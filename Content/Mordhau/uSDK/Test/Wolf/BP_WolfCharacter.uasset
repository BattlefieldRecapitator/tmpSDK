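; BP_WolfCharacter is a test wolf character for Mordhau that can follow players and punishes its killer.
; Interacting with it tells its WolfController to follow that Mordhau character.
; Basic axis inputs and the space bar also allow direct movement, look and jumping.
; On death it ragdolls and, if a player controller killed it, plays a sound at world origin and deals heavy damage to that player's Mordhau character.
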(event EventBeginPlay)

(event EventOnKilled
  (params (EventInstigator :type Controller%20Object%20Reference))
  (Class|AdvancedCharacter|StartRagdoll)
  (bind _asmordhau_player_controller (Utilities|Casting|CastToMordhauPlayerController EventInstigator))
  (Audio|PlaySoundatLocation "/Game/Mordhau/uSDK/Test/Wolf/wolf5.wolf5" "0, 0, 0" "0, 0, 0" 1.0 1.0 0.0 0 0 0)
  (bind _asbp_mordhau_character (Utilities|Casting|CastToBP_MordhauCharacter (Pawn|GetControlledPawn _asmordhau_player_controller)))
  (Game|Damage|ApplyDamage _asbp_mordhau_character 99.0 0 0 "/Script/Engine.DamageType"))

(event EventOnInteractionStart
  (params (Character :type Advanced%20Character%20Object%20Reference))
  (bind _aswolf_controller (Utilities|Casting|CastToWolfController (Pawn|GetController)))
  (bind _asbp_mordhau_character (Utilities|Casting|CastToBP_MordhauCharacter Character))
  (Default|Follow _aswolf_controller _asbp_mordhau_character))

(event Input|AxisEvents|InputAxisMoveForward
  (params (AxisValue :type Float%20%28single-precision%29))
  (bind _returnvalue (Pawn|GetControlRotation :!class /Script/Engine.Pawn))
  (bind (_roll _pitch _yaw) (Math|Rotator|BreakRotator _returnvalue))
  ;[1 1 1] Placeheld By TheMattman
  (Pawn|Input|AddMovementInput (Math|Vector|GetForwardVector (Math|Rotator|MakeRotator 0.0 _pitch _yaw)) AxisValue false))

(event Input|AxisEvents|InputAxisMoveRight
  (params (AxisValue :type Float%20%28single-precision%29))
  (bind _returnvalue (Pawn|GetControlRotation :!class /Script/Engine.Pawn))
  (bind (_roll _pitch _yaw) (Math|Rotator|BreakRotator _returnvalue))
  ;[1 1 1] Placeheld By TheMattman
  (Pawn|Input|AddMovementInput (Math|Vector|GetRightVector (Math|Rotator|MakeRotator 0.0 _pitch _yaw)) AxisValue false))

(event Input|AxisEvents|InputAxisTurn
  (params (AxisValue :type Float%20%28single-precision%29))
  ;[1 1 1] Placeheld By TheMattman
  (Pawn|Input|AddControllerYawInput (Pawn|GetControlledPawn (Pawn|GetController)) AxisValue))

(event Input|AxisEvents|InputAxisLookUp
  (params (AxisValue :type Float%20%28single-precision%29))
  ;[1 1 1] Placeheld By TheMattman
  (Pawn|Input|AddControllerPitchInput (Pawn|GetControlledPawn (Pawn|GetController)) AxisValue))

(event Input|KeyboardEvents|SpaceBar
  (params (Key :type Key%20Structure))
  ;[1 1 1] Placeheld By TheMattman
  (:Pressed
    (Character|Jump)))

(fn ConstructionScript
  (|CallParentFunction))