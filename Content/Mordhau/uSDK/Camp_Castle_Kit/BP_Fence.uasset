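; BP_Fence is a spline-based fence placement actor for the Camp Castle Kit.
; Its construction script selects a static mesh from the FenceStyle choice, covering wooden, stone, metal and prop variants.
; It then adds a spline mesh component between each pair of neighbouring spline points, bent along their positions and tangents on the chosen forward axis, with query and physics collision.
; The event graph has no active logic.
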(event EventBeginPlay
  (|CallParentFunction) ; This node is disabled and will not be called.\nDrag off pins to build functionality.
)

(event Collision|EventActorBeginOverlap
  (params (OtherActor :type Actor%20Object%20Reference)))

(event EventTick
  (params (DeltaSeconds :type Float%20%28single-precision%29))
  (|CallParentFunction DeltaSeconds) ; This node is disabled and will not be called.\nDrag off pins to build functionality.
)

(fn ConstructionScript
  (bind _spline (Variables|Default|GetSpline))
  (|CallParentFunction)
  (switch Utilities|FlowControl|Switch|SwitchonEFences (Variables|Default|GetFence%20Style)
    (:NewEnumerator0
      (Variables|Default|Setstaticmesh "/Game/MedievalVillage/Models/WoodFence_mdl.WoodFence_mdl"))
    (:NewEnumerator1
      (Variables|Default|Setstaticmesh "/Game/Mordhau/Maps/TaigaMap/Taiga_Merged_Assets/WaterfallShackFence.WaterfallShackFence"))
    (:NewEnumerator2
      (Variables|Default|Setstaticmesh "/Game/Mordhau/Maps/TaigaMap/Taiga_Merged_Assets/StoneFence02.StoneFence02"))
    (:NewEnumerator3
      (Variables|Default|Setstaticmesh "/Game/Mordhau/Maps/TaigaMap/Taiga_Merged_Assets/StoneFence03.StoneFence03"))
    (:NewEnumerator4
      (Variables|Default|Setstaticmesh "/Game/Mordhau/Maps/TaigaMap/Taiga_Merged_Assets/StoneFence04.StoneFence04"))
    (:NewEnumerator5
      (Variables|Default|Setstaticmesh "/Game/Mordhau/Maps/TaigaMap/Taiga_Merged_Assets/StoneFence05.StoneFence05"))
    (:NewEnumerator6
      (Variables|Default|Setstaticmesh "/Game/Mordhau/Assets/Environment/Props/SmallProps/StaticMeshes/MetalFence.MetalFence"))
    (:NewEnumerator7
      (Variables|Default|Setstaticmesh "/Game/Mordhau/Assets/Environment/Props/SmallProps/StaticMeshes/prop_fence_02.prop_fence_02")))
  (for _index (range 0 (- (Spline|GetNumberOfSplinePoints _spline) 2))
    (bind _returnvalue (AddComponent|AddSplineMeshComponent false))
    (Components|StaticMesh|SetStaticMesh _returnvalue (Variables|Default|Getstaticmesh))
    (SplineMesh|SetForwardAxis _returnvalue (Variables|Default|GetForwardAxis) true)
    (Utilities|Array|AddUnique (Variables|Default|GetSegments) _returnvalue)
    (Transformation|AttachComponentToComponent _returnvalue _spline "None" "KeepRelative" "KeepRelative" "KeepRelative" true)
    (SplineMesh|SetStartandEnd _returnvalue (Spline|GetLocationatSplinePoint _spline _index "Local") (Spline|GetTangentatSplinePoint _spline _index "Local") (Spline|GetLocationatSplinePoint _spline (+ _index 1) "Local") (Spline|GetTangentatSplinePoint _spline (+ _index 1) "Local") true :!class /Script/Engine.SplineMeshComponent)
    (Collision|SetCollisionEnabled _returnvalue "QueryAndPhysics")))