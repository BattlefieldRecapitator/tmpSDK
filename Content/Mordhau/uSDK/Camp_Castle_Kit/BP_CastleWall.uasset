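; Castle wall Blueprint from the Camp Castle Kit that builds a wall along an editable spline.
; The construction script adds a colliding spline mesh for each span between neighboring points, matched to its positions and tangents, with only the first point forced to linear.
; A light, normal or dark style picks the wall mesh, and an optional gate swaps the segment at a chosen index to a barbican gate mesh.
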(event EventBeginPlay
  (|CallParentFunction) ; This node is disabled and will not be called.\nDrag off pins to build functionality.
)

(event Collision|EventActorBeginOverlap
  (params (OtherActor :type Actor%20Object%20Reference)))

(event EventTick
  (params (DeltaSeconds :type Float%20%28single-precision%29))
  (|CallParentFunction DeltaSeconds) ; This node is disabled and will not be called.\nDrag off pins to build functionality.
)

(fn ConstructionScript
  (bind _spline (Variables|Default|GetSpline))
  (|CallParentFunction)
  (Spline|SetSplinePointType (Variables|Default|GetSpline) 0 "Linear" true)
  (Variables|Default|SetSegments (Utilities|Array|MakeArray 0))
  (switch Utilities|FlowControl|Switch|SwitchonEWalls (Variables|Default|GetWall%20Style)
    (:NewEnumerator0
      (Variables|Default|Setstaticmesh "/Game/Mordhau/Maps/AndrewG_Testing_Map/Andrews_Art_Tests/Assets/Castle/Castle_Meshes/Modules/Crossroads/Castle_wall_01_c.Castle_wall_01_c"))
    (:NewEnumerator1
      (Variables|Default|Setstaticmesh "/Game/Mordhau/Maps/AndrewG_Testing_Map/Andrews_Art_Tests/Assets/Castle/Castle_Meshes/Modules/castle_wall_01.castle_wall_01"))
    (:NewEnumerator2
      (Variables|Default|Setstaticmesh "/Game/Mordhau/Maps/AndrewG_Testing_Map/Andrews_Art_Tests/Assets/Castle/Castle_Meshes/Modules/castle_wall_01_b.castle_wall_01_b")))
  (for _index (range 0 (- (Spline|GetNumberOfSplinePoints _spline) 2))
    (bind _returnvalue (AddComponent|AddSplineMeshComponent false))
    (Components|StaticMesh|SetStaticMesh _returnvalue (Variables|Default|Getstaticmesh))
    (SplineMesh|SetForwardAxis _returnvalue (Variables|Default|GetForwardAxis) true)
    (Utilities|Array|AddUnique (Variables|Default|GetSegments) _returnvalue)
    (Transformation|AttachComponentToComponent _returnvalue _spline "None" "KeepRelative" "KeepRelative" "KeepRelative" true)
    (SplineMesh|SetStartandEnd _returnvalue (Spline|GetLocationatSplinePoint _spline _index "Local") (Spline|GetTangentatSplinePoint _spline _index "Local") (Spline|GetLocationatSplinePoint _spline (+ _index 1) "Local") (Spline|GetTangentatSplinePoint _spline (+ _index 1) "Local") true :!class /Script/Engine.SplineMeshComponent)
    (Collision|SetCollisionEnabled _returnvalue "QueryAndPhysics"))
  (if (Variables|Default|GetGate)
    (Components|StaticMesh|SetStaticMesh (Utilities|Array|Get(acopy) (Variables|Default|GetSegments) (Variables|Default|GetGateIndex)) "/Game/Mordhau/Maps/AndrewG_Testing_Map/Andrews_Art_Tests/Assets/Castle/Castle_Meshes/Modules/castle_barbican_gate.castle_barbican_gate")))