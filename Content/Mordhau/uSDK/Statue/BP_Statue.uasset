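; BP_Statue places a posed Mordhau character in the level as a statue.
; On BeginPlay it spawns a BP_MordhauCharacter at SpawnPoint and applies the profile from its Templar function, with equipment, through the Mordhau singleton.
; It then makes the character immune to damage and overrides its mesh animation with a kite-shield standing pose.
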(event EventBeginPlay
  (bind _spawn_point (Variables|Default|GetSpawn%20point))
  (bind _returnvalue (Transformation|GetWorldTransform _spawn_point))
  (bind _returnvalue_2 (Game|SpawnActorfromClass "/Game/Mordhau/Blueprints/Characters/BP_MordhauCharacter.BP_MordhauCharacter_C" (Math|Transform|MakeTransform (.location _returnvalue) (.rotation _returnvalue) (.scale _returnvalue)) "AlwaysSpawn" 0 0))
  (Class|MordhauSingleton|ApplyProfileto (Class|MordhauUtilityLibrary|GetMordhauSingleton) (Utilities|Templar) _returnvalue_2 0 true)
  (Variables|/Script/Engine.Actor|SetbCanBeDamaged _returnvalue_2 false)
  (Components|Animation|OverrideAnimationData (Variables|/Script/Engine.Character|GetMesh _returnvalue_2) "/Game/Mordhau/Animations/RawClips/Misc/Poses/Pose_KiteShieldStand.Pose_KiteShieldStand" true true 0.0 1.0))

(fn ConstructionScript)