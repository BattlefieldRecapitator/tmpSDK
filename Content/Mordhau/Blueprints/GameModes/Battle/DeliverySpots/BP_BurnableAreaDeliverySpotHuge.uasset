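; A huge burnable-area delivery spot for Battle game modes that shows a fire growing as its visual stage progresses.
; Each ProgressVisualStage event switches on VisualStage, playing a fire hit sound, raising the post-process blend weight and activating that stage's effects.
; Across seven stages it layers in fire, smoke and GPU flare effects, with a second fire sound introduced and then volume-adjusted early on.
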(event EventBeginPlay
  (|CallParentFunction) ; This node is disabled and will not be called.\nDrag off pins to build functionality.
)

(event Collision|EventActorBeginOverlap
  (params (OtherActor :type Actor%20Object%20Reference))
  (|CallParentFunction OtherActor) ; This node is disabled and will not be called.\nDrag off pins to build functionality.
)

(event EventTick
  (params (DeltaSeconds :type Float%20%28single-precision%29))
  (|CallParentFunction DeltaSeconds) ; This node is disabled and will not be called.\nDrag off pins to build functionality.
)

(event EventProgressVisualStage
  (bind _fire2sound (Variables|Default|GetFire2Sound))
  (switch int (Variables|Default|GetVisualStage)
    (:0
      (Variables|/Script/Engine.PostProcessComponent|SetBlendWeight (Variables|Default|GetPostProcess) 0.1)
      (Audio|Components|Audio|Play (Variables|Default|GetSC_FireHitSound) 0.0)
      (Components|Activation|Activate (Variables|Default|GetFire1) false))
    (:1
      (Variables|/Script/Engine.PostProcessComponent|SetBlendWeight (Variables|Default|GetPostProcess) 0.3)
      (Audio|Components|Audio|Play (Variables|Default|GetSC_FireHitSound) 0.0)
      (Components|Activation|Activate (Variables|Default|GetFire2) false)
      (Components|Activation|Activate _fire2sound false)
      (Components|Activation|Activate (Variables|Default|GetGpuFlares) false))
    (:2
      (Variables|/Script/Engine.PostProcessComponent|SetBlendWeight (Variables|Default|GetPostProcess) 0.5)
      (Audio|Components|Audio|Play (Variables|Default|GetSC_FireHitSound) 0.0)
      (Components|Activation|Activate (Variables|Default|GetFire3) false)
      (Components|Activation|Activate (Variables|Default|GetSmoke) false)
      (Audio|Components|Audio|AdjustVolume _fire2sound 0.0 1.0 :!class /Script/Engine.AudioComponent))
    (:3
      (Variables|/Script/Engine.PostProcessComponent|SetBlendWeight (Variables|Default|GetPostProcess) 0.6)
      (Audio|Components|Audio|Play (Variables|Default|GetSC_FireHitSound) 0.0)
      (Components|Activation|Activate (Variables|Default|GetGpuFlares2) false))
    (:4
      (Variables|/Script/Engine.PostProcessComponent|SetBlendWeight (Variables|Default|GetPostProcess) 0.7)
      (Audio|Components|Audio|Play (Variables|Default|GetSC_FireHitSound) 0.0)
      (Components|Activation|Activate (Variables|Default|GetFire4) false))
    (:5
      (Variables|/Script/Engine.PostProcessComponent|SetBlendWeight (Variables|Default|GetPostProcess) 0.9)
      (Audio|Components|Audio|Play (Variables|Default|GetSC_FireHitSound) 0.0)
      (Components|Activation|Activate (Variables|Default|GetGpuFlares3) false))
    (:6
      (Variables|/Script/Engine.PostProcessComponent|SetBlendWeight (Variables|Default|GetPostProcess) 1.0)
      (Audio|Components|Audio|Play (Variables|Default|GetSC_FireHitSound) 0.0)
      (Components|Activation|Activate (Variables|Default|GetFire6) false))))

(fn ConstructionScript
  (|CallParentFunction))