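; Base destroyable for the Frontline hero objective, judging by its name, that tracks damage stages as its health drops.
; When replicated health changes, it scans DamageMeshesHealth and stores the last index whose threshold is at or above current health in BestDamageIdx.
; It then calls UpdateAnimInstance, which is empty here and likely a hook for child Blueprints, before running the parent handler.
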(event EventBeginPlay
  (|CallParentFunction) ; This node is disabled and will not be called.\nDrag off pins to build functionality.
)

(event Collision|EventActorBeginOverlap
  (params (OtherActor :type Actor%20Object%20Reference))
  (|CallParentFunction OtherActor) ; This node is disabled and will not be called.\nDrag off pins to build functionality.
)

(event EventTick
  (params (DeltaSeconds :type Float%20%28single-precision%29))
  (|CallParentFunction DeltaSeconds) ; This node is disabled and will not be called.\nDrag off pins to build functionality.
)

(event EventOnReplicatedHealthChanged
  (Utilities|FlowControl|Sequence
    (:then_0
      (for (_array_element _array_index) (Variables|Default|GetDamageMeshesHealth)
        (if (<= (Variables|Default|GetReplicatedHealth) _array_element)
          (Variables|Default|SetBestDamageIdx _array_index))))
    (:then_1
      (CallFunction|UpdateAnimInstance))
    (:then_2
      (|CallParentFunction))))

(fn ConstructionScript
  (|CallParentFunction))

(fn UpdateAnimInstance)