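; Explosive barrel deliverable for Battle game modes that breaks apart when it thuds.
; OnThud runs the parent logic, then the authority destroys the deliverable collision component.
; Without an authority check, it also clears the skeletal mesh and spawns keg-breaking particles and sound at the barrel's location, using the valid-mesh test so this only happens while the mesh is still set.
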(event EventBeginPlay)

(event Collision|EventActorBeginOverlap
  (params (OtherActor :type Actor%20Object%20Reference)))

(event EventTick
  (params (DeltaSeconds :type Float%20%28single-precision%29)))

(event EventOnThud
  (bind _returnvalue (Transformation|GetActorLocation))
  (bind _skeletalmeshcomponent (Variables|Default|GetSkeletalMeshComponent))
  (bind _deliverablecollision (Variables|Default|GetDeliverableCollision))
  (|CallParentFunction)
  (Utilities|FlowControl|Sequence
    (:then_0
      (Networking|SwitchHasAuthority
        (:Authority
          (Utilities|IsValid _deliverablecollision
            (:Is%20Valid
              (Components|DestroyComponent _deliverablecollision))))))
    (:then_1
      (Utilities|IsValid (Variables|/Script/Engine.SkinnedMeshComponent|GetSkeletalMesh _skeletalmeshcomponent)
        (:Is%20Valid
          (Class|SkinnedMeshComponent|SetSkeletalMesh _skeletalmeshcomponent 0 true)
          (Effects|SpawnEmitteratLocation "/Game/StarterContent/Particles/KegBreaking.KegBreaking" _returnvalue (Transformation|GetActorRotation))
          (Audio|SpawnSoundatLocation "/Game/Mordhau/Audio/Cues/Siege/SC_BarrelBreaking.SC_BarrelBreaking" _returnvalue "0, 0, 0" 1.0 1.0 0.0 0 0))))))

(fn ConstructionScript
  (|CallParentFunction))