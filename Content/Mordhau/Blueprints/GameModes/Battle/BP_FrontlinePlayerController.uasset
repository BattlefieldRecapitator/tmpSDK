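; Frontline mode player controller that handles offers to take part in an objective and shows the objectives HUD.
; An offer triggers an on-screen announcement, and the team select key then declines it instead of opening team select.
; Possessing a pawn with no prior vehicle time either resets the offer flags and overrides widget visibility for a kill objective, or reveals objectives once the match has started.
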(event Custom|NotifyOfferedParticipation
  (bind _hud (Variables|Default|GetHUD))
  (Variables|Default|SetOfferedParticipation true)
  (if (Pawn|IsLocalPlayerController)
    (Utilities|IsValid _hud
      (:Is%20Valid
        (Default|ShowAnnouncement _hud "You have been chosen to participate in the objective" (Class|MordhauUtilityLibrary|FormatText (Utilities|Text|MakeLiteralText "Press [{Action_Show Team Select}] to decline")) 6.0)))))

(event Custom|DeclineParticipation
  (Variables|Default|SetDeclinedObjectiveParticipation true))

(event EventBeginPlay
  (|CallParentFunction) ; This node is disabled and will not be called.\nDrag off pins to build functionality.
)

(event EventTick
  (params (DeltaSeconds :type Float%20%28single-precision%29))
  (|CallParentFunction DeltaSeconds) ; This node is disabled and will not be called.\nDrag off pins to build functionality.
)

(event EventOnAfterPossess
  (params (APawn :type Pawn%20Object%20Reference))
  (Utilities|FlowControl|Sequence
    (:then_0
      (bind _asmordhau_character (Utilities|Casting|CastToMordhauCharacter APawn))
      (if (== (Variables|/Script/Mordhau.MordhauCharacter|GetLastVehicleTime _asmordhau_character) 0.0)
        (bind _asbp_frontline_kill_objective (Utilities|Casting|CastToBP_FrontlineKillObjective APawn)
          (:then
            (Variables|/Script/Mordhau.MordhauWidgetComponent|SetOverrideVisible (Variables|/Game/Mordhau/Blueprints/GameModes/Battle/BP_FrontlineKillObjective.BP_FrontlineKillObjective_C|GetMordhauWidget _asbp_frontline_kill_objective) 0)
            (Variables|Default|SetDeclinedObjectiveParticipation false)
            (Variables|Default|SetOfferedParticipation false))
          (:CastFailed
            (bind _asbp_frontline_hud (Utilities|Casting|CastToBP_FrontlineHUD (Class|MordhauUtilityLibrary|GetMordhauHUD)))
            (bind _asbp_frontline_game_state (Utilities|Casting|CastToBP_FrontlineGameState (Game|GetGameState)))
            (if (Class|GameStateBase|HasMatchStarted _asbp_frontline_game_state)
              (if (not (Widget|IsVisible (Variables|/Game/Mordhau/Blueprints/BP_MordhauHUD.BP_MordhauHUD_C|GetObjectives _asbp_frontline_hud)))
                (Default|ShowObjectives _asbp_frontline_hud)))))))
    (:then_1
      (|CallParentFunction APawn))))

(event Input|ActionEvents|InputActionShowTeamSelect
  (params (Key :type Key%20Structure))
  (bind _hud (Variables|Default|GetHUD))
  (:Pressed
    (if (Variables|Default|GetOfferedParticipation)
      (if (Variables|Default|GetDeclinedObjectiveParticipation)
        (CallFunction|HandleTeamSelect :!label _label)
        (else
          (Variables|Default|SetDeclinedObjectiveParticipation true)
          (CallFunction|DeclineParticipation)
          (Utilities|IsValid _hud
            (:Is%20Valid
              (Default|ShowAnnouncement _hud "Declined objective participation" "" 2.0)))))
      (else
        (goto _label)))))

(fn ConstructionScript
  (|CallParentFunction))