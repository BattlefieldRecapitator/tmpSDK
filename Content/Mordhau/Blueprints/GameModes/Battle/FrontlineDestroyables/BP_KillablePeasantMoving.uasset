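; Moving killable peasant for Frontline destroyables that loops along a referenced spline until its health reaches zero, when it stops ticking.
; Position and yaw derive each tick from server world time, spline length and move speed, keeping movement in step across machines without accumulated state.
; On the server, a short vertical trace at the mesh applies massive damage to any destroyable actor or deployable ballista it hits.
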(event Collision|EventActorBeginOverlap
  (params (OtherActor :type Actor%20Object%20Reference))
  (|CallParentFunction OtherActor) ; This node is disabled and will not be called.\nDrag off pins to build functionality.
)

(event EventTick
  (params (DeltaSeconds :type Float%20%28single-precision%29))
  (bind _returnvalue (Game|GetGameState))
  (bind _skeletalmesh (Variables|Default|GetSkeletalMesh))
  (bind _spline (Variables|Default|GetSpline))
  (bind _returnvalue_2 (Transformation|GetWorldLocation _skeletalmesh))
  (bind _spline_2 (Variables|/Game/Mordhau/Blueprints/Interactables/BP_SplineActor.BP_SplineActor_C|GetSpline _spline))
  (bind _returnvalue_3 (Spline|GetSplineLength _spline_2))
  (|CallParentFunction DeltaSeconds)
  (Utilities|IsValid _returnvalue
    (:Is%20Valid
      (if (== (Variables|Default|GetReplicatedHealth) 0)
        (Actor|Tick|SetActorTickEnabled false)
        (else
          (Variables|Default|SetTrack (Math|Float|%(Float) (/ (GameState|GetServerWorldTimeSeconds _returnvalue) (/ _returnvalue_3 (Variables|Default|GetMoveSpeed))) 1.0))
          (Transformation|SetActorLocationAndRotation self (Spline|GetLocationatDistanceAlongSpline _spline_2 (Math|Float|Lerp 0.0 _returnvalue_3 (Variables|Default|GetTrack)) "World") (Math|Rotator|MakeRotator 0.0 0.0 (- (.Yaw (Math|Rotator|BreakRotator (Spline|GetRotationatDistanceAlongSpline _spline_2 (Math|Float|Lerp 0.0 _returnvalue_3 (Variables|Default|GetTrack)) "World"))) 9e+01)))
          (Networking|SwitchHasAuthority
            (:Authority
              (bind (_outhit _returnvalue_4) (Collision|LineTraceForObjects (+ _returnvalue_2 "0, 0,150.000000") _returnvalue_2 (Variables|Default|GetObjectTypesToTrace) false 0 "None"))
              (if _returnvalue_4
                (bind _asbp_destroyable_actor (Utilities|Casting|CastToBP_DestroyableActor (.HitActor (Collision|BreakHitResult _outhit)))
                  (:then
                    (Game|Damage|ApplyDamage _asbp_destroyable_actor 9999.0 0 0))
                  (:CastFailed
                    (bind _asbp_deployable_ballista (Utilities|Casting|CastToBP_DeployableBallista (.HitActor (Collision|BreakHitResult _outhit))))
                    (Game|Damage|ApplyDamage _asbp_deployable_ballista 9999.0 0 0)))))))))))

(fn ConstructionScript
  (|CallParentFunction))