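; Killable peasant actor in the Frontline destroyables folder, playing a configurable looping or one-off animation until killed.
; On replicated health drops, the authority stores the last hit normal and location for replication, while the material's blood intensity rises and a blood splash spawns at the hit.
; At zero health it plays a sound, ragdolls with a hit impulse, dissolves via material parameters, then hides and disables collision.
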(event EventBeginPlay
  (|CallParentFunction)
  (Utilities|FlowControl|Sequence
    (:then_0
      (Networking|SwitchHasAuthority
        (:Authority
          (Variables|/Script/Engine.SkinnedMeshComponent|SetMeshComponentUpdateFlag (Variables|Default|GetSkeletalMesh) "AlwaysTickPoseAndRefreshBones"))))
    (:then_1
      (Components|Timeline|SetPlayRate (Variables|Default|GetSkeletalMesh) (Variables|Default|GetAnimationPlayRate)))))

(event Collision|EventActorBeginOverlap
  (params (OtherActor :type Actor%20Object%20Reference))
  (|CallParentFunction OtherActor) ; This node is disabled and will not be called.\nDrag off pins to build functionality.
)

(event EventTick
  (params (DeltaSeconds :type Float%20%28single-precision%29))
  (|CallParentFunction DeltaSeconds) ; This node is disabled and will not be called.\nDrag off pins to build functionality.
)

(event EventOnReplicatedHealthChanged
  (bind _returnvalue (Math|Float|MakeLiteralFloat 1e+01))
  (bind _replicatedhealth (Variables|Default|GetReplicatedHealth))
  (bind _skeletalmesh (Variables|Default|GetSkeletalMesh))
  (bind _skeletalmesh_2 (Variables|Default|GetSkeletalMesh))
  (bind _lastdamagenormal (Variables|Default|GetLastDamageNormal))
  (bind _lastdamagelocation (Variables|Default|GetLastDamageLocation))
  (bind (_x _y _z) (Math|Vector|BreakVector _lastdamagenormal))
  (bind (_x_2 _y_2 _z_2) (Math|Vector|BreakVector _lastdamagelocation))
  (Utilities|FlowControl|Sequence
    (:then_0
      (if (< _replicatedhealth (Variables|Default|GetLastReplicatedHealth))
        (Utilities|FlowControl|Sequence
          (:then_0
            (Networking|SwitchHasAuthority
              (:Authority
                (Variables|Default|SetReplicatedLastHitNormal (Math|Vector|MakeVectorNetQuantizeNormal _x _y _z))
                (Variables|Default|SetReplicatedLastHitLocation (Math|Vector|MakeVectorNetQuantize _x_2 _y_2 _z_2)))))
          (:then_1
            (bind _returnvalue_2 (Rendering|Material|CreateDynamicMaterialInstance (Variables|Default|GetSkeletalMesh) 0 0 "None" :!class /Script/Engine.PrimitiveComponent))
            (Rendering|Material|SetScalarParameterValue _returnvalue_2 "BloodIntensity" (- 1.0 (/ (Math|Conversions|ToFloat(Byte) (Variables|Default|GetReplicatedHealth)) 1e+02)) :!class /Script/Engine.MaterialInstanceDynamic))
          (:then_2
            (Game|SpawnActorfromClass "/Game/Mordhau/Blueprints/BP_BloodSplash.BP_BloodSplash_C" (Math|Transform|MakeTransform (Math|Transform|TransformLocation (Transformation|GetActorTransform) (Variables|Default|GetReplicatedLastHitLocation))) "Undefined" 0 0)
            (if (== _replicatedhealth 0)
              (Audio|PlaySoundatLocation 0 (Transformation|GetSocketLocation (Variables|Default|GetSkeletalMesh) "Head") "0, 0, 0" 1.0 1.0 0.0 0 0 0)
              (Collision|SetCollisionProfileName _skeletalmesh "Ragdoll" :!class /Script/Engine.PrimitiveComponent)
              (Class|SkeletalMeshComponent|SetAllBodiesSimulatePhysics _skeletalmesh true)
              (Class|PrimitiveComponent|AddForceatLocation _skeletalmesh (* (Variables|Default|GetReplicatedLastHitNormal) -1e+06) (Math|Transform|TransformLocation (Transformation|GetActorTransform) (Variables|Default|GetReplicatedLastHitLocation)) "None")
              (bind _returnvalue_3 (Rendering|Material|CreateDynamicMaterialInstance (Variables|Default|GetSkeletalMesh) 0 0 "None" :!class /Script/Engine.PrimitiveComponent))
              (Rendering|Material|SetScalarParameterValue _returnvalue_3 "DissolveDuration" _returnvalue :!class /Script/Engine.MaterialInstanceDynamic)
              (Rendering|Material|SetScalarParameterValue _returnvalue_3 "DissolveStartTime" (Utilities|Time|GetTimeSeconds) :!class /Script/Engine.MaterialInstanceDynamic)
              (Utilities|FlowControl|Delay _returnvalue)
              (Development|SetHiddeninGame _skeletalmesh_2 true true)
              (Collision|SetCollisionEnabled _skeletalmesh_2 "NoCollision")
              (Variables|/Script/Engine.SkinnedMeshComponent|SetMeshComponentUpdateFlag (Variables|Default|GetSkeletalMesh) "OnlyTickPoseWhenRendered"))))))
    (:then_1
      (|CallParentFunction))))

(fn ConstructionScript
  (|CallParentFunction)
  (Components|Animation|OverrideAnimationData (Variables|Default|GetSkeletalMesh) (Variables|Default|GetInitialAnimation) true true 0.0 1.0))