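; Battle-mode interactable spawn point that hands out deliverable items tied to a capture point.
; Interaction spawns the deliverable and equips it on the character, tracking it on success or destroying it on failure.
; CanInteract refuses the capture point's owning team and anyone already holding a deliverable in the right hand.
; Activate shows the marker with a team restriction derived from the owner; Disable hides it and destroys all tracked deliverables.
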(event EventBeginPlay)

(event Collision|EventActorBeginOverlap
  (params (OtherActor :type Actor%20Object%20Reference)))

(event EventTick
  (params (DeltaSeconds :type Float%20%28single-precision%29)))

(event EventOnInteractionStart
  (params (Character :type Mordhau%20Character%20Object%20Reference))
  (Utilities|IsValid Character
    (:Is%20Valid
      (bind _returnvalue (Game|SpawnActorfromClass (Variables|Default|GetDeliverableClass) (Transformation|GetActorTransform) "Undefined" 0 0))
      (bind _returnvalue_2 (Class|MordhauCharacter|PickUp Character _returnvalue))
      (if _returnvalue_2
        (Utilities|Array|Add (Variables|Default|GetSpawnedDeliverables) _returnvalue)
        (else
          (Actor|DestroyActor _returnvalue))))))

(fn ConstructionScript)

(fn CanInteract
  (params (Character :type Mordhau%20Character%20Object%20Reference))
  (bind _capturepoint (Variables|Default|GetCapturePoint))
  (Utilities|IsValid Character
    (:Is%20Valid
      (Utilities|IsValid _capturepoint
        (:Is%20Valid
          (if (!= (Variables|/Script/Mordhau.AdvancedCharacter|GetTeam Character) (Variables|/Script/Mordhau.ControlPoint|GetOwningTeam _capturepoint))
            (Utilities|Casting|CastToBP_DeliverableEquipment (Variables|/Script/Mordhau.MordhauCharacter|GetRightHandEquipment Character)
              (:then
                (return false))
              (:CastFailed
                _))
            (else
              (return false))))
        (:Is%20Not%20Valid
          _)))
    (:Is%20Not%20Valid
      _))
  (return (stale _returnvalue)))

(fn Activate
  (bind _mordhauwidget (Variables|Default|GetMordhauWidget))
  (Variables|Default|SetbIsInteractable true)
  (Variables|/Script/Mordhau.MordhauWidgetComponent|SetOverrideVisible _mordhauwidget -1)
  (Variables|/Script/Mordhau.MordhauWidgetComponent|SetViewTargetTeamRestriction _mordhauwidget (Math|Conversions|ToInteger(Byte) (Utilities|Select :Index (Variables|/Script/Mordhau.ControlPoint|GetOwningTeam (Variables|Default|GetCapturePoint)) :Option%200 1 :Option%201 0))))

(fn Disable
  (Variables|Default|SetbIsInteractable false)
  (Variables|/Script/Mordhau.MordhauWidgetComponent|SetOverrideVisible (Variables|Default|GetMordhauWidget) 0)
  (for _array_element (Variables|Default|GetSpawnedDeliverables)
    (Utilities|IsValid _array_element
      (:Is%20Valid
        (Actor|DestroyActor _array_element))))
  (Utilities|Array|Clear (Variables|Default|GetSpawnedDeliverables)))