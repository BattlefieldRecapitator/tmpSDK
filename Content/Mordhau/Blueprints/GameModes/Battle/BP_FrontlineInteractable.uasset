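; Frontline mode objective interactable tied to a capture point, which the team not owning that point completes through held interactions.
; It shows when the enemy gains prerequisites and hides when they are lost, the point's progress is full, or required interactions are reached.
; The authority counts interactions and awards score; the replicated count updates the point's weighted progress and floating widget.
; The widget icon switches between defence and objective by local team.
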(event Custom|OnInteractionsChanged)

(event Custom|ProgressVisualStage)

(event EventOnHeldInteractionStart
  (params (Character :type Mordhau%20Character%20Object%20Reference))
  (Utilities|IsValid Character
    (:Is%20Valid
      (bind _asmordhau_player_controller (Utilities|Casting|CastToMordhauPlayerController (Pawn|GetController Character)))
      (CallFunction|IncrementInteractions _asmordhau_player_controller))))

(event Collision|EventActorBeginOverlap
  (params (OtherActor :type Actor%20Object%20Reference)))

(event EventTick
  (params (DeltaSeconds :type Float%20%28single-precision%29)))

(event EventOnInitialize
  (params (Point :type BP%20Capture%20Point%20Object%20Reference))
  (CallFunction|Initialize Point))

(event EventOnEnemyGainedPrerequisites
  (CallFunction|EnemyGainedPrerequisites)
  (CallFunction|UpdateUIWidgets))

(event EventOnEnemyLostPrerequisites
  (CallFunction|EnemyLostPrerequisites)
  (CallFunction|UpdateUIWidgets))

(event EventOnUpdateUIWidgets
  (CallFunction|UpdateUIWidgets))

(event EventOnAnyObjectiveProgressChanged
  (bind _capturepoint (Variables|Default|GetCapturePoint))
  (Utilities|IsValid _capturepoint
    (:Is%20Valid
      (if (== (Variables|/Game/Mordhau/Blueprints/GameModes/Battle/BP_CapturePoint.BP_CapturePoint_C|GetObjectiveProgress _capturepoint) 1.0)
        (CallFunction|EnemyLostPrerequisites)))))

(fn ConstructionScript
  (|CallParentFunction))

(fn Activate
  (if (< (Variables|Default|GetInteractions) (Variables|Default|GetRequiredInteractions))
    (Variables|Default|SetbIsInteractable true)
    (Variables|/Script/Mordhau.MordhauWidgetComponent|SetOverrideVisible (Variables|Default|GetMordhauWidget) -1)
    (Development|SetHiddeninGame (Variables|Default|GetDecal) false false)))

(fn Disable
  (Variables|Default|SetbIsInteractable false)
  (Variables|/Script/Mordhau.MordhauWidgetComponent|SetOverrideVisible (Variables|Default|GetMordhauWidget) 0)
  (Development|SetHiddeninGame (Variables|Default|GetDecal) true false))

(fn Initialize
  (params (CapturePoint :type BP%20Capture%20Point%20Object%20Reference))
  (Variables|Default|SetCapturePoint CapturePoint))

(fn EnemyGainedPrerequisites
  (bind _capturepoint (Variables|Default|GetCapturePoint))
  (Utilities|IsValid _capturepoint
    (:Is%20Valid
      (if (not (== (Variables|/Game/Mordhau/Blueprints/GameModes/Battle/BP_CapturePoint.BP_CapturePoint_C|GetObjectiveProgress _capturepoint) 1.0))
        (if (< (Variables|Default|GetInteractions) (Variables|Default|GetRequiredInteractions))
          (CallFunction|Activate))))))

(fn EnemyLostPrerequisites
  (CallFunction|Disable))

(fn OnRepInteractions
  (bind _capturepoint (Variables|Default|GetCapturePoint))
  (Utilities|FlowControl|Sequence
    (:then_0
      (if (>= (Variables|Default|GetInteractions) (Variables|Default|GetRequiredInteractions))
        (CallFunction|Disable)))
    (:then_1
      (Utilities|IsValid _capturepoint
        (:Is%20Valid
          (Default|ObjectivesChanged _capturepoint)
          (bind _asbp_interact_widget_floater (Utilities|Casting|CastToBP_InteractWidgetFloater (UserInterface|GetUserWidgetObject (Variables|Default|GetMordhauWidget))))
          (bind _progress (CallFunction|GetObjectiveProgress))
          (Default|UpdateProgress _asbp_interact_widget_floater (- 1.0 _progress)))))
    (:then_2
      (CallFunction|OnInteractionsChanged))))

(fn IncrementInteractions
  (params (Interactor :type Mordhau%20Player%20Controller%20Object%20Reference))
  (Networking|SwitchHasAuthority
    (:Authority
      (if (< (Variables|Default|GetInteractions) (Variables|Default|GetRequiredInteractions))
        (Utilities|FlowControl|Sequence
          (:then_0
            (Utilities|IsValid Interactor
              (:Is%20Valid
                (Class|MordhauPlayerController|GiveClientScoreBP Interactor "Objective" (Variables|Default|GetScoreAwardPerInteract)))))
          (:then_1
            (Variables|Default|SetInteractions (+ (Variables|Default|GetInteractions) 1))))))))

(fn CanInteract
  (params (Character :type Mordhau%20Character%20Object%20Reference))
  (return false))

(fn CanHeldInteract
  (params (Character :type Mordhau%20Character%20Object%20Reference))
  (bind _capturepoint (Variables|Default|GetCapturePoint))
  (Utilities|IsValid _capturepoint
    (:Is%20Valid
      (Utilities|IsValid Character
        (:Is%20Valid
          (if (!= (Variables|/Script/Mordhau.AdvancedCharacter|GetTeam Character) (Variables|/Script/Mordhau.ControlPoint|GetOwningTeam _capturepoint))
            _
            (else
              (return false))))
        (:Is%20Not%20Valid
          _)))
    (:Is%20Not%20Valid
      _))
  (return (stale _returnvalue)))

(fn UpdateUIWidgets
  (bind _capturepoint (Variables|Default|GetCapturePoint))
  (bind _mordhauwidget (Variables|Default|GetMordhauWidget))
  (Utilities|IsValid _capturepoint
    (:Is%20Valid
      (if (not (== (Variables|/Game/Mordhau/Blueprints/GameModes/Battle/BP_CapturePoint.BP_CapturePoint_C|GetObjectiveProgress _capturepoint) 1.0))
        (Utilities|IsValid _mordhauwidget
          (:Is%20Valid
            (bind _asbp_interact_widget_floater (Utilities|Casting|CastToBP_InteractWidgetFloater (UserInterface|GetUserWidgetObject _mordhauwidget)))
            (bind _asmordhau_game_state (Utilities|Casting|CastToMordhauGameState (Game|GetGameState)))
            (bind _asmordhau_player_state (Utilities|Casting|CastToMordhauPlayerState (Variables|/Script/Engine.Controller|GetPlayerState (Game|GetPlayerController 0))))
            (if (== (Variables|/Script/Mordhau.ControlPoint|GetOwningTeam _capturepoint) (Math|Conversions|ToByte(Integer) (Variables|/Script/Mordhau.MordhauPlayerState|GetTeam _asmordhau_player_state)))
              (Class|Image|SetBrush (Variables|/Game/Mordhau/Blueprints/GameModes/Battle/BP_InteractWidgetFloater.BP_InteractWidgetFloater_C|GetIcon _asbp_interact_widget_floater) (Utilities|Struct|MakeSlateBrush "(X=36.000000,Y=40.000000)" "(Left=0.000000,Top=0.000000,Right=0.000000,Bottom=0.000000)" (Utilities|Struct|MakeSlateColor "(R=0.848958,G=0.848958,B=0.848958,A=1.000000)") "/Game/Mordhau/UI/UIAssets/Textures/ic_defence_lvl1.ic_defence_lvl1" "Image" "NoTile" "NoMirror"))
              (else
                (Class|Image|SetBrush (Variables|/Game/Mordhau/Blueprints/GameModes/Battle/BP_InteractWidgetFloater.BP_InteractWidgetFloater_C|GetIcon _asbp_interact_widget_floater) (Utilities|Struct|MakeSlateBrush "(X=32.000000,Y=32.000000)" "(Left=0.000000,Top=0.000000,Right=0.000000,Bottom=0.000000)" "(SpecifiedColor=(R=1.000000,G=1.000000,B=1.000000,A=1.000000),ColorUseRule=UseColor_Specified)" (Variables|Default|GetObjectiveIcon) "Image" "NoTile" "NoMirror"))))))))))

(fn GetObjectiveProgress
  (return (* (/ (Math|Conversions|ToFloat(Byte) (Variables|Default|GetInteractions)) (Math|Conversions|ToFloat(Byte) (Variables|Default|GetRequiredInteractions))) (Variables|Default|GetObjectiveWeight))))