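; Invasion-mode pushable minecart that rides a spline and blows up on arrival, collapsing a cave.
; On cosmetic-capable instances, Tick turns spline progress into wheel rotation and move speed for the anim instance, using paired DoOnce gates to fade rolling audio.
; Arrival runs fuse sparks and sound, then after a delay swaps the cart for rubble and triggers explosion effects, radial damage with knockback, and camera shakes.
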(event EventTick
  (params (DeltaSeconds :type Float%20%28single-precision%29))
  (bind _progress (Variables|Default|GetProgress))
  (bind _targetsplineactor (Variables|Default|GetTargetSplineActor))
  (bind _wheelssound (Variables|Default|GetWheelsSound))
  (bind _spline (Variables|/Game/Mordhau/Blueprints/Interactables/BP_SplineActor.BP_SplineActor_C|GetSpline _targetsplineactor))
  (bind _returnvalue (Spline|GetSplineLength _spline))
  (|CallParentFunction DeltaSeconds)
  (Networking|CanExecuteCosmeticEvents
    (:True
      (if (not (Math|Float|NearlyEqual(Float) DeltaSeconds 0.0 1e-06))
        (Utilities|FlowControl|Sequence
          (:then_0
            (bind _asab_mine_cart (Utilities|Casting|CastToAB_MineCart (Components|SkeletalMesh|GetAnimInstance (Variables|Default|GetSkeletalMesh))))
            (Variables|/Game/Mordhau/Animations/Blueprints/AB_MineCart.AB_MineCart_C|SetWheels _asab_mine_cart (Math|Rotator|MakeRotator (* (/ (* _returnvalue _progress) 95.0) 3.6e+02) 0.0 0.0))
            (bind _output_get (Variables|/Game/Mordhau/Animations/Blueprints/AB_MineCart.AB_MineCart_C|SetMoveSpeed _asab_mine_cart (/ (* _returnvalue (- _progress (Variables|Default|GetPreviousProgress))) DeltaSeconds)))
            (if (> _output_get 1.0)
              (Utilities|FlowControl|DoOnce false :!label _label
                (:Completed
                  (Audio|Components|Audio|FadeIn _wheelssound 1.0 1.0 0.0 :!class /Script/Engine.AudioComponent)
                  (goto _label_2 Reset)))
              (else
                (Utilities|FlowControl|DoOnce false :!label _label_2
                  (:Completed
                    (Audio|Components|Audio|FadeOut _wheelssound 0.2 0.0 :!class /Script/Engine.AudioComponent)
                    (goto _label Reset))))))
          (:then_1
            (Variables|Default|SetPreviousProgress (Variables|Default|GetProgress))))))))

(event EventPushableArrivedatDestination
  (bind _returnvalue (Transformation|GetActorLocation))
  (Components|Activation|Activate (Variables|Default|GetP_ExplosiveSpark1) false)
  (Audio|Components|Audio|Play (Variables|Default|GetSC_ExplosiveBarrelFuse) 0.0)
  (Utilities|FlowControl|Delay 5.0)
  (Components|Activation|Deactivate (Variables|Default|GetP_ExplosiveSpark1))
  (Development|SetHiddeninGame (Variables|Default|GetRubblePile05) false true)
  (Development|SetHiddeninGame (Variables|Default|GetSkeletalMesh) true false)
  (Components|Activation|Activate (Variables|Default|GetP_CatapultImpact) false)
  (Class|MordhauUtilityLibrary|MordhauApplyRadialDamagewithFalloff 2.5e+03 3e+01 0.0 0.0 (Transformation|GetWorldLocation (Variables|Default|GetP_Explosion)) 6e+02 1e+03 6.0 0 1.2e+04 9e+03 1.4e+03 self 0 "ECC_Visibility" false)
  (Camera|PlayWorldCameraShake "/Game/Mordhau/Blueprints/CameraShakes/ExplosionShake.ExplosionShake_C" _returnvalue 1e+03 1e+04)
  (Camera|PlayWorldCameraShake "/Game/Mordhau/Blueprints/CameraShakes/CollapseRumble.CollapseRumble_C" _returnvalue 1e+03 4e+03)
  (Audio|Components|Audio|Play (Variables|Default|GetSC_FallingCaveRumble1) 0.0))

(fn ConstructionScript
  (|CallParentFunction))