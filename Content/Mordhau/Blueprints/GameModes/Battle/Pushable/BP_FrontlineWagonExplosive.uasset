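; Explosive wagon pushable for Frontline mode that blows up after it arrives at its destination.
; On arrival, spark particles and a fuse sound run during a short delay, then give way to explosion, smoke and debris effects with audio.
; The blast hides the wagon and keg meshes, disables skeletal mesh collision, reveals a decal and shakes nearby cameras.
; A radial damage and knockback call is present but unconnected, so this graph deals no damage.
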(event EventBeginPlay
  (|CallParentFunction) ; This node is disabled and will not be called.\nDrag off pins to build functionality.
)

(event Collision|EventActorBeginOverlap
  (params (OtherActor :type Actor%20Object%20Reference))
  (|CallParentFunction OtherActor) ; This node is disabled and will not be called.\nDrag off pins to build functionality.
)

(event EventTick
  (params (DeltaSeconds :type Float%20%28single-precision%29))
  (|CallParentFunction DeltaSeconds) ; This node is disabled and will not be called.\nDrag off pins to build functionality.
)

(event EventPushableArrivedatDestination
  (bind _p_explosivespark (Variables|Default|GetP_ExplosiveSpark))
  (bind _p_explosion (Variables|Default|GetP_Explosion))
  (Components|Activation|Activate _p_explosivespark false)
  (Utilities|FlowControl|Delay 5.0)
  (Components|Activation|Deactivate _p_explosivespark)
  (Components|Activation|Activate _p_explosion false)
  (Collision|SetCollisionEnabled (Variables|Default|GetSkeletalMesh) "NoCollision")
  (Rendering|SetVisibility (Variables|Default|GetSkeletalMesh) false false)
  (Rendering|SetVisibility (Variables|Default|GetDecal1) true false)
  (Camera|PlayWorldCameraShake 0 (Transformation|GetWorldLocation _p_explosion) 1e+03 1e+04))

(fn ConstructionScript
  (|CallParentFunction))