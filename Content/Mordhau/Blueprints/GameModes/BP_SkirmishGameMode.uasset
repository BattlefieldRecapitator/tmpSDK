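; Skirmish game mode: a round-based team elimination mode where the first team to reach the round-win target takes the match.
; Tick drives a waiting, start, play and end state machine stored in the game state, timed by server world time.
; Round start resets world actors and clears pawns; play closes late spawning and blocks dead players from respawning.
; Rounds end on timeout or one team remaining, scoring the team with most survivors unless drawn.
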(event EventOnKilled
  (params (Killer :type Controller%20Object%20Reference) (KilledPlayer :type Controller%20Object%20Reference) (KilledPawn :type Pawn%20Object%20Reference) (Type :type EMordhauDamageType%20Enum :default "Generic") (SubType :type Byte :default 0) (DamageSource :type Actor%20Object%20Reference) (DamageAgent :type Actor%20Object%20Reference))
  (Utilities|FlowControl|Sequence
    (:then_0
      (if (Class|GameMode|IsMatchinProgress)
        (Utilities|Array|Add (Variables|Default|GetAlreadyDiedArray) KilledPlayer)))
    (:then_1
      (|CallParentFunction Killer KilledPlayer KilledPawn Type SubType DamageSource DamageAgent))))

(event EventBeginPlay
  (|CallParentFunction))

(event EventTick
  (params (DeltaSeconds :type Float%20%28single-precision%29))
  (if (Class|GameMode|IsMatchinProgress)
    (bind _asbp_skirmish_game_state (Utilities|Casting|CastToBP_SkirmishGameState (Game|GetGameState)))
    (switch Utilities|FlowControl|Switch|SwitchonE_SkirmishRoundStage (.Stage (Utilities|Struct|BreakSTRUCT_SkirmishRoundInfo (Variables|/Game/Mordhau/Blueprints/GameModes/BP_SkirmishGameState.BP_SkirmishGameState_C|GetRoundInfo _asbp_skirmish_game_state)))
      (:WaitingforPlayers
        (Utilities|Array|Clear (Variables|Default|GetAlreadyDiedArray))
        (bind _return (CallFunction|CanStartRound))
        (if _return
          (CallFunction|StartRoundStart)))
      (:RoundStart
        (if (>= (GameState|GetServerWorldTimeSeconds _asbp_skirmish_game_state) (+ (.StartTime (Utilities|Struct|BreakSTRUCT_SkirmishRoundInfo (Variables|/Game/Mordhau/Blueprints/GameModes/BP_SkirmishGameState.BP_SkirmishGameState_C|GetRoundInfo _asbp_skirmish_game_state))) (Variables|/Game/Mordhau/Blueprints/GameModes/BP_SkirmishGameState.BP_SkirmishGameState_C|GetRoundStartDuration _asbp_skirmish_game_state)))
          (bind _return_2 (CallFunction|CanStartRound))
          (if _return_2
            (CallFunction|StartRound)
            (else
              (CallFunction|StartWaitingforPlayers)))))
      (:RoundPlay
        (if (>= (GameState|GetServerWorldTimeSeconds _asbp_skirmish_game_state) (+ (.StartTime (Utilities|Struct|BreakSTRUCT_SkirmishRoundInfo (Variables|/Game/Mordhau/Blueprints/GameModes/BP_SkirmishGameState.BP_SkirmishGameState_C|GetRoundInfo _asbp_skirmish_game_state))) (Variables|/Game/Mordhau/Blueprints/GameModes/BP_SkirmishGameState.BP_SkirmishGameState_C|GetRoundDuration _asbp_skirmish_game_state)))
          (CallFunction|EndRound :!label _label)
          (else
            (Utilities|FlowControl|Sequence
              (:then_0
                (if (>= (GameState|GetServerWorldTimeSeconds _asbp_skirmish_game_state) (+ (.StartTime (Utilities|Struct|BreakSTRUCT_SkirmishRoundInfo (Variables|/Game/Mordhau/Blueprints/GameModes/BP_SkirmishGameState.BP_SkirmishGameState_C|GetRoundInfo _asbp_skirmish_game_state))) (Variables|/Game/Mordhau/Blueprints/GameModes/BP_SkirmishGameState.BP_SkirmishGameState_C|GetLateRoundSpawnDuration _asbp_skirmish_game_state)))
                  (Variables|/Script/Mordhau.MordhauGameState|SetbAllowSpawning _asbp_skirmish_game_state false)))
              (:then_1
                (bind _return_3 (CallFunction|MoreThanOneTeamAlive))
                (if (not _return_3)
                  (goto _label)))))))
      (:RoundEnd
        (bind _return_4 (CallFunction|CanStartRound))
        (if _return_4
          (if (>= (GameState|GetServerWorldTimeSeconds _asbp_skirmish_game_state) (+ (.StartTime (Utilities|Struct|BreakSTRUCT_SkirmishRoundInfo (Variables|/Game/Mordhau/Blueprints/GameModes/BP_SkirmishGameState.BP_SkirmishGameState_C|GetRoundInfo _asbp_skirmish_game_state))) (Variables|/Game/Mordhau/Blueprints/GameModes/BP_SkirmishGameState.BP_SkirmishGameState_C|GetRoundEndDuration _asbp_skirmish_game_state)))
            (CallFunction|StartRoundStart))
          (else
            (CallFunction|StartWaitingforPlayers)))))))

(fn ConstructionScript
  (|CallParentFunction))

(fn StartRoundStart
  (Variables|Default|SetbIsScoringDisabled true)
  (bind _asbp_skirmish_game_state (Utilities|Casting|CastToBP_SkirmishGameState (Game|GetGameState)))
  (Utilities|FlowControl|Sequence
    (:then_0
      (bind _outactors (Actor|GetAllActorsOfClass "/Script/Mordhau.MordhauActor"))
      (for _array_element _outactors
        (Utilities|IsValid _array_element
          (:Is%20Valid
            (bind _asmordhau_equipment (Utilities|Casting|CastToMordhauEquipment _array_element)
              (:then
                (if (Variables|/Script/Mordhau.MordhauEquipment|GetbAllowCleanup _asmordhau_equipment)
                  (Utilities|Casting|CastToBP_CharacterDoll (Class|MordhauEquipment|GetParentCharacter _asmordhau_equipment)
                    (:CastFailed
                      (Actor|DestroyActor _asmordhau_equipment)))))
              (:CastFailed
                (bind _asmordhau_projectile (Utilities|Casting|CastToMordhauProjectile _array_element)
                  (:then
                    (Actor|DestroyActor _asmordhau_projectile))
                  (:CastFailed
                    (bind _asbp_destroyable_actor (Utilities|Casting|CastToBP_DestroyableActor _array_element))
                    (Default|SetHealth _asbp_destroyable_actor (Variables|/Game/Mordhau/Blueprints/Interactables/Environment/BP_DestroyableActor.BP_DestroyableActor_C|GetSpawnHealth _asbp_destroyable_actor))
                    (bind _asbp_door (Utilities|Casting|CastToBP_Door _asbp_destroyable_actor))
                    (Variables|/Game/Mordhau/Blueprints/Interactables/Environment/BP_Door.BP_Door_C|SetDoorState _asbp_door (Variables|/Game/Mordhau/Blueprints/Interactables/Environment/BP_Door.BP_Door_C|GetStartingState _asbp_door))))))))))
    (:then_1
      (Utilities|Array|Clear (Variables|Default|GetAlreadyDiedArray))
      (Variables|/Script/Mordhau.MordhauGameState|SetRoundInfo _asbp_skirmish_game_state (Utilities|Struct|MakeSTRUCT_SkirmishRoundInfo "RoundStart" 0 (GameState|GetServerWorldTimeSeconds (Game|GetGameState))))
      (Variables|/Script/Mordhau.MordhauGameState|SetbAllowSpawning _asbp_skirmish_game_state true)
      (bind _outactors_2 (Actor|GetAllActorsOfClass "/Script/Engine.Controller"))
      (for _array_element_2 _outactors_2
        (bind _asmordhau_player_state (Utilities|Casting|CastToMordhauPlayerState (Variables|/Script/Engine.Controller|GetPlayerState _array_element_2)))
        (if (>= (Variables|/Script/Mordhau.MordhauPlayerState|GetTeam _asmordhau_player_state) 0)
          (CallFunction|UnpossessandDestroyPawn _array_element_2 false))))))

(fn EndRound
  (Utilities|FlowControl|Sequence
    (:then_0
      (bind _asbp_skirmish_game_state (Utilities|Casting|CastToBP_SkirmishGameState (Game|GetGameState)))
      (bind _returnvalue (Class|MordhauGameState|GetPlayerCountsPerTeam _asbp_skirmish_game_state true false))
      (if (.bFoundDraw (Class|MordhauUtilityLibrary|GetMaxIndexwithDraw _returnvalue))
        (LocalVariables|SetWinner 255)
        (Variables|/Game/Mordhau/Blueprints/GameModes/BP_SkirmishGameState.BP_SkirmishGameState_C|SetRoundInfo _asbp_skirmish_game_state (Utilities|Struct|MakeSTRUCT_SkirmishRoundInfo "RoundEnd" (LocalVariables|GetWinner) (GameState|GetServerWorldTimeSeconds (Game|GetGameState))) :!label _label)
        (Variables|/Script/Mordhau.MordhauGameState|SetbAllowSpawning _asbp_skirmish_game_state false)
        (else
          (LocalVariables|SetWinner (Math|Conversions|ToByte(Integer) (.ReturnValue (Class|MordhauUtilityLibrary|GetMaxIndexwithDraw _returnvalue))))
          (Class|MordhauGameMode|AddTeamScore (Math|Conversions|ToInteger(Byte) (LocalVariables|GetWinner)) 1.0)
          (if (>= (Utilities|Array|Get(acopy) (Variables|/Script/Mordhau.MordhauGameState|GetTeamScores _asbp_skirmish_game_state) (Math|Conversions|ToInteger(Byte) (LocalVariables|GetWinner))) (Math|Conversions|ToFloat(Integer) (Variables|Default|GetWinConditionRounds)))
            (Class|GameMode|EndMatch)
            (Variables|/Game/Mordhau/Blueprints/GameModes/BP_MordhauGameState.BP_MordhauGameState_C|SetMatchEndInfo _asbp_skirmish_game_state (Utilities|Struct|MakeSTRUCT_MatchEndInfo 0 (Math|Conversions|ToInteger(Byte) (LocalVariables|GetWinner)) (Utilities|Array|Get(acopy) (Variables|/Script/Mordhau.MordhauGameState|GetTeamScores _asbp_skirmish_game_state) (Math|Conversions|ToInteger(Byte) (LocalVariables|GetWinner)))))
            (else
              (goto _label))))))
    (:then_1
      (Variables|Default|SetbIsScoringDisabled true))))

(fn MoreThanOneTeamAlive
  (bind _asbp_skirmish_game_state (Utilities|Casting|CastToBP_SkirmishGameState (Game|GetGameState)))
  (if (Variables|/Script/Mordhau.MordhauGameState|GetbAllowSpawning _asbp_skirmish_game_state)
    (return true)
    (else
      (bind _returnvalue (Class|MordhauGameState|GetPlayerCountsPerTeam _asbp_skirmish_game_state true false))
      (for _array_element _returnvalue
        (if (> _array_element 0)
          (if (LocalVariables|GetFoundLivingTeam)
            (return true)
            (else
              (LocalVariables|SetFoundLivingTeam true)))))
      (return false))))

(fn ControllerCanRestart
  (params (Controller :type Controller%20Object%20Reference))
  (bind _returnvalue (|CallParentFunction Controller))
  (return (and _returnvalue (not (Utilities|Array|ContainsItem (Variables|Default|GetAlreadyDiedArray) Controller)))))

(fn StartWaitingforPlayers
  (Variables|Default|SetbIsScoringDisabled true)
  (bind _asbp_skirmish_game_state (Utilities|Casting|CastToBP_SkirmishGameState (Game|GetGameState)))
  (Utilities|Array|Clear (Variables|Default|GetAlreadyDiedArray))
  (Variables|/Game/Mordhau/Blueprints/GameModes/BP_SkirmishGameState.BP_SkirmishGameState_C|SetRoundInfo _asbp_skirmish_game_state (Utilities|Struct|MakeSTRUCT_SkirmishRoundInfo "WaitingforPlayers" 0 (Utilities|Time|GetTimeSeconds)))
  (Variables|/Script/Mordhau.MordhauGameState|SetbAllowSpawning _asbp_skirmish_game_state true))

(fn CanStartRound
  (bind _asbp_skirmish_game_state (Utilities|Casting|CastToBP_SkirmishGameState (Game|GetGameState)))
  (bind _returnvalue (Class|MordhauGameState|GetPlayerCountsPerTeam _asbp_skirmish_game_state false true))
  (for _array_element _returnvalue
    (if (> _array_element 0)
      (if (LocalVariables|GetFoundFirstTeam)
        (return true)
        (else
          (LocalVariables|SetFoundFirstTeam true)))))
  (return false))

(fn StartRound
  (Variables|Default|SetbIsScoringDisabled false)
  (bind _asbp_skirmish_game_state (Utilities|Casting|CastToBP_SkirmishGameState (Game|GetGameState)))
  (Utilities|Array|Clear (Variables|Default|GetAlreadyDiedArray))
  (Variables|/Game/Mordhau/Blueprints/GameModes/BP_SkirmishGameState.BP_SkirmishGameState_C|SetRoundInfo _asbp_skirmish_game_state (Utilities|Struct|MakeSTRUCT_SkirmishRoundInfo "RoundPlay" 0 (GameState|GetServerWorldTimeSeconds (Game|GetGameState)))))