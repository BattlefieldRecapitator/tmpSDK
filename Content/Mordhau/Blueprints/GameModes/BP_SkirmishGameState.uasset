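; Game state for Mordhau's round-based Skirmish mode, presenting round flow and match results on the HUD.
; Tick shows waiting and countdown announcements; duplicated RoundInfo rep-notifies announce round winners and clear corpses and non-environmental-fire fields on authority at round start.
; Overrides derive the scoreboard timer from stage and server time, label the objective "Wins", hide spawn info, and gate input and profile changes by stage.
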(event EventHandleMatchEndInfo
  (|CallParentFunction)
  (bind _asbp_mordhau_hud (Utilities|Casting|CastToBP_MordhauHUD (Class|MordhauUtilityLibrary|GetMordhauHUD)))
  (bind _asmordhau_player_state (Utilities|Casting|CastToMordhauPlayerState (Variables|/Script/Engine.Controller|GetPlayerState (Game|GetPlayerController 0))))
  (if (or (== (Variables|/Script/Mordhau.MordhauPlayerState|GetTeam _asmordhau_player_state) (.WinnerTeam (Utilities|Struct|BreakSTRUCT_MatchEndInfo (Variables|Default|GetMatchEndInfo)))) (== (Variables|/Script/Mordhau.MordhauPlayerState|GetTeam _asmordhau_player_state) -1))
    (Default|ShowMatchResult _asbp_mordhau_hud true "victory")
    (else
      (Default|ShowMatchResult _asbp_mordhau_hud false "defeat"))))

(event EventTick
  (params (DeltaSeconds :type Float%20%28single-precision%29))
  (bind _returnvalue (GameState|GetServerWorldTimeSeconds))
  (bind _returnvalue_2 (Game|GetPlayerController 0))
  (bind _roundstartduration (Variables|Default|GetRoundStartDuration))
  (bind _roundinfo_tmp (Variables|Default|GetRoundInfo_tmp))
  (bind _starttime (Utilities|Struct|BreakSTRUCT_SkirmishRoundInfo _roundinfo_tmp))
  (bind _returnvalue_3 (+ _starttime _roundstartduration))
  (bind _returnvalue_4 (- _returnvalue_3 _returnvalue))
  (bind _returnvalue_5 (Math|Float|Ceil _returnvalue_4))
  (|CallParentFunction DeltaSeconds)
  (Utilities|Casting|CastToBP_MordhauPlayerController _returnvalue_2)
  (if (Pawn|IsLocalPlayerController _returnvalue_2)
    (bind _asbp_mordhau_hud (Utilities|Casting|CastToBP_MordhauHUD (HUD|GetHUD _returnvalue_2)))
    (if (Utilities|Name|Equal(Name) (Variables|Default|GetMatchState) "InProgress")
      (switch Utilities|FlowControl|Switch|SwitchonE_SkirmishRoundStage (Variables|Default|GetLastObservedRoundStage_0)
        (:NewEnumerator0
          (Default|ShowAnnouncement _asbp_mordhau_hud "Waiting for players" "" 0.1))
        (:NewEnumerator1
          (if (!= _returnvalue_5 0)
            (Default|ShowAnnouncement _asbp_mordhau_hud "Round starting" (Utilities|Text|FormatText "-{0}-" _returnvalue_5) 0.1)))))))

(event EventBeginPlay)

(fn ConstructionScript
  (|CallParentFunction))

(fn OnRepRoundInfo
  (bind _roundinfo_tmp (Variables|Default|GetRoundInfo_tmp))
  (bind _roundendduration (Variables|Default|GetRoundEndDuration))
  (bind (_stage _winner) (Utilities|Struct|BreakSTRUCT_SkirmishRoundInfo _roundinfo_tmp))
  (if (Utilities|Enum|NotEqual(Enum) _stage (LocalVariables|GetLastObservedRoundStage_tmp))
    (bind _output_get (LocalVariables|SetLastObservedRoundStage_tmp _stage))
    (switch Utilities|FlowControl|Switch|SwitchonE_SkirmishRoundStage _output_get
      (:RoundStart
        (Utilities|FlowControl|Sequence
          (:then_0
            ;[1 1 1] Destroy ragdoll corpses
            (bind _outactors (Actor|GetAllActorsOfClass "/Script/Mordhau.AdvancedCharacter"))
            (for _array_element _outactors
              (if (and (Ability|HasAuthority _array_element) (Variables|/Script/Mordhau.MordhauCharacter|GetbIsDead _array_element))
                (Actor|DestroyActor _array_element))))
          (:then_1
            ;[1 1 1] Destroy master fields
            (bind _outactors_2 (Actor|GetAllActorsOfClass "/Script/Mordhau.MasterField"))
            (for _array_element_2 _outactors_2
              (Utilities|Casting|CastToBP_EnvFireField _array_element_2
                (:CastFailed
                  (if (Ability|HasAuthority _array_element_2)
                    (Actor|DestroyActor _array_element_2))))))))
      (:RoundEnd
        (bind _asbp_mordhau_hud (Utilities|Casting|CastToBP_MordhauHUD (Class|MordhauUtilityLibrary|GetMordhauHUD)))
        (if (== _winner 255)
          (Default|ShowAnnouncement _asbp_mordhau_hud "Draw!" "" _roundendduration)
          (else
            (bind _returnvalue (Class|MordhauGameState|GetTeamName (Math|Conversions|ToInteger(Byte) _winner)))
            (Default|ShowAnnouncement _asbp_mordhau_hud (Utilities|Text|FormatText "{a} has won the round." (Utilities|Text|ToText(String) _returnvalue)) "" _roundendduration)))))))

(fn GetScoreboardTimeinProgress
  (bind _returnvalue (GameState|GetServerWorldTimeSeconds))
  (bind _roundinfo_tmp (Variables|Default|GetRoundInfo_tmp))
  (bind (_stage _winner _starttime) (Utilities|Struct|BreakSTRUCT_SkirmishRoundInfo _roundinfo_tmp))
  (switch Utilities|FlowControl|Switch|SwitchonE_SkirmishRoundStage _stage
    (:WaitingforPlayers
      (return (Math|Timespan|MakeTimespan 200)))
    (:RoundStart
      (return (Math|Timespan|FromSeconds (Math|Float|Max(Float) (- (+ _starttime (Variables|Default|GetRoundStartDuration)) _returnvalue) 0.0))))
    (:RoundPlay
      (return (Math|Timespan|FromSeconds (Math|Float|Max(Float) (- (+ _starttime (Variables|Default|GetRoundDuration)) _returnvalue) 0.0))))
    (:RoundEnd
      (return (Math|Timespan|FromSeconds (Math|Float|Max(Float) (- (+ _starttime (Variables|Default|GetRoundEndDuration)) _returnvalue) 0.0))))))

(fn GetScoreboardObjectiveName
  (return "Wins"))

(fn ShouldHideSpawnInfoText
  (return true))

(fn ShouldBlockPawnInput
  (bind _returnvalue (|CallParentFunction))
  (return (or _returnvalue (Utilities|Enum|Equal(Enum) (Variables|Default|GetLastObservedRoundStage_0) "NewEnumerator1"))))

(fn CanImmediatelyChangeProfile
  (params (Controller :type Controller%20Object%20Reference))
  (bind _returnvalue (|CallParentFunction Controller))
  (return (or _returnvalue (Utilities|Enum|Equal(Enum) (Variables|Default|GetLastObservedRoundStage_0) "NewEnumerator1"))))

(fn OnRepRoundInfoTmp
  (bind _roundinfo_tmp (Variables|Default|GetRoundInfo_tmp))
  (bind _roundendduration (Variables|Default|GetRoundEndDuration))
  (bind (_stage _winner) (Utilities|Struct|BreakSTRUCT_SkirmishRoundInfo _roundinfo_tmp))
  (if (Utilities|Enum|NotEqual(Enum) _stage (Variables|Default|GetLastObservedRoundStagetmp2))
    (bind _output_get (Variables|Default|SetLastObservedRoundStagetmp2 _stage))
    (switch Utilities|FlowControl|Switch|SwitchonE_SkirmishRoundStage _output_get
      (:RoundStart
        (Utilities|FlowControl|Sequence
          (:then_0
            ;[1 1 1] Destroy ragdoll corpses
            (bind _outactors (Actor|GetAllActorsOfClass "/Script/Mordhau.AdvancedCharacter"))
            (for _array_element _outactors
              (if (and (Ability|HasAuthority _array_element) (Variables|/Script/Mordhau.MordhauCharacter|GetbIsDead _array_element))
                (Actor|DestroyActor _array_element))))
          (:then_1
            ;[1 1 1] Destroy master fields
            (bind _outactors_2 (Actor|GetAllActorsOfClass "/Script/Mordhau.MasterField"))
            (for _array_element_2 _outactors_2
              (Utilities|Casting|CastToBP_EnvFireField _array_element_2
                (:CastFailed
                  (if (Ability|HasAuthority _array_element_2)
                    (Actor|DestroyActor _array_element_2))))))))
      (:RoundEnd
        (bind _asbp_mordhau_hud (Utilities|Casting|CastToBP_MordhauHUD (Class|MordhauUtilityLibrary|GetMordhauHUD)))
        (if (== _winner 255)
          (Default|ShowAnnouncement _asbp_mordhau_hud "Draw!" "" _roundendduration)
          (else
            (bind _returnvalue (Class|MordhauGameState|GetTeamName (Math|Conversions|ToInteger(Byte) _winner)))
            (Default|ShowAnnouncement _asbp_mordhau_hud (Utilities|Text|FormatText "{a} has won the round." (Utilities|Text|ToText(String) _returnvalue)) "" _roundendduration)))))))