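; BP_Medpack is a throwable medpack that becomes a limited-use healing bag once thrown.
; Throwing unloads it on the server, recording the thrower; the unloaded state swaps in an open-bag mesh and turns held interaction into "Heal".
; Heals cap at 100 health and respect the character's healing-disable flag.
; The thrower earns scaled score for healing friendlies, and the bag destroys itself when uses run out.
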(event EventFireProjectile
  (params (Origin :type Vector%20%28by%20ref%29 :default "0, 0, 0") (Orientation :type Rotator%20%28by%20ref%29 :default "0, 0, 0") (OwningController :type Controller%20Object%20Reference) (ExpectedDelay :type Float%20%28single-precision%29))
  (|CallParentFunction Origin Orientation OwningController ExpectedDelay)
  (Networking|SwitchHasAuthority
    (:Authority
      (Class|MordhauEquipment|SetLoaded false)
      (Variables|Default|SetThrowerController OwningController))))

(event EventOnHeldInteractionStart
  (params (Character :type Mordhau%20Character%20Object%20Reference))
  (if (Variables|Default|GetbIsLoaded)
    (|CallParentFunction Character)
    (else
      (CallFunction|ApplyHeal Character))))

(event EventOnLoadedChanged
  (|CallParentFunction)
  (if (not (Variables|Default|GetbIsLoaded))
    (Variables|Default|SetOriginalMaxHoldTime (Variables|Default|GetMaxInteractionHoldTime))
    (Variables|Default|SetMaxInteractionHoldTime (Variables|Default|GetHealTimeToHold))
    (Variables|Default|SetHeldInteractionText "Heal")
    (Class|SkinnedMeshComponent|SetSkeletalMesh (Variables|Default|GetSkeletalMeshComponent) "/Game/Mordhau/Assets/Weapons/ThrownExplosives/Bag/OpenBag.OpenBag" true)
    (Variables|Default|SetRagdollStayTime 1.2e+02)))

(fn ConstructionScript)

(fn CanInteract
  (params (Character :type Mordhau%20Character%20Object%20Reference))
  (if (Variables|Default|GetbIsLoaded)
    (return (stale _returnvalue))
    (else
      (return false))))

(fn CanHeldInteract
  (params (Character :type Mordhau%20Character%20Object%20Reference))
  (if (Variables|Default|GetbIsLoaded)
    (return (stale _returnvalue))
    (else
      (Utilities|IsValid Character
        (:Is%20Valid
          (return (and (< (Variables|/Script/Mordhau.AdvancedCharacter|GetHealth Character) 100) (not (Variables|/Script/Mordhau.AdvancedCharacter|GetbDisableHealingItems Character)))))
        (:Is%20Not%20Valid
          (return true))))))

(fn ApplyHeal
  (params (Character :type Mordhau%20Character%20Object%20Reference))
  (bind _output_get (LocalVariables|SetToHeal (Math|Integer|Min(Integer) (- 100 (Math|Conversions|ToInteger(Byte) (Variables|/Script/Mordhau.AdvancedCharacter|GetHealth Character))) (Variables|Default|GetHealthPerHeal))))
  (if (> _output_get 0)
    (LocalVariables|SetScoreToGive (Math|Float|Truncate (* _output_get (Variables|Default|GetHealScoreModifier))))
    (Utilities|FlowControl|Sequence
      (:then_0
        (Class|AdvancedCharacter|OffsetHealth Character (LocalVariables|GetToHeal) true)
        (bind _asmordhau_player_controller (Utilities|Casting|CastToMordhauPlayerController (Variables|Default|GetThrowerController)))
        (bind _asmordhau_game_state (Utilities|Casting|CastToMordhauGameState (Game|GetGameState)))
        (bind _returnvalue (Class|MordhauGameState|IsFriendly _asmordhau_game_state _asmordhau_player_controller Character))
        (if (and _returnvalue (> (LocalVariables|GetScoreToGive) 0))
          (Class|MordhauPlayerController|GiveClientScoreBP _asmordhau_player_controller "Heal" (LocalVariables|GetScoreToGive))))
      (:then_1
        (bind _output_get_2 (Variables|Default|SetHealsLeft (- (Variables|Default|GetHealsLeft) 1)))
        (if (<= _output_get_2 0)
          (Actor|DestroyActor))))))