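; Explosive barrel equipment that starts a short fuse when its loaded state changes, then explodes.
; The change blocks holstering, and the server records the controller of the carrying Mordhau character, vehicle included, as instigator.
; After the delay the server applies radial damage around the barrel credited to that controller, then destroys the actor.
; Mode switching is always refused, and debug strings print at fuse start and detonation.
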(event EventBeginPlay)

(event EventActorBeginOverlap
  (params (OtherActor :type Actor%20Object%20Reference)))

(event EventTick
  (params (DeltaSeconds :type Float%20%28single-precision%29)))

(event EventOnLoadedChanged
  (|CallParentFunction)
  (Development|PrintString "Going to blow up")
  (Variables|Default|SetbCanHolster false)
  (Networking|SwitchHasAuthority
    (:Authority
      (Utilities|FlowControl|Sequence
        (:then_0
          (bind _asmordhau_character (Utilities|Casting|CastToMordhauCharacter (Class|MordhauUtilityLibrary|GetAttachParentActor)))
          (bind _returnvalue (Class|MordhauCharacter|GetControllerIncludingVehicle _asmordhau_character))
          (Variables|Default|SetInstigatorController_0 _returnvalue))
        (:then_1
          (Utilities|FlowControl|Delay 3.0)
          (Development|PrintString "BOOM!")
          (Game|Damage|ApplyRadialDamage 1.5e+02 (Transformation|GetActorLocation) 5e+02 "/Script/Engine.DamageType" 0 self (Variables|Default|GetInstigatorController_0) false "ECC_Visibility")
          (Actor|DestroyActor))))))

(fn ConstructionScript)

(fn OnRequestModeSwitch
  (params (Character :type Mordhau%20Character%20Object%20Reference))
  (return false))