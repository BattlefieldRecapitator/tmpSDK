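; Two-handed rock projectile that does full damage only when falling fast, such as when dropped from height.
; Before the parent processes a hit, it maps vertical velocity to a clamped damage multiplier, leaving slow-falling or flat throws at a small fraction of damage.
; Head kills, and cosmetic head hits on already-dead characters, queue a blunt-force dismemberment on the character.
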(event EventOnUsedtoKillOther
  (params (Character :type Advanced%20Character%20Object%20Reference) (Type :type EMordhauDamageType%20Enum :default "Generic") (SubType :type Byte :default 0) (bone :type Name%20%28by%20ref%29 :default "None") (Point :type Vector%20%28by%20ref%29 :default "0, 0, 0") (Source :type Actor%20Object%20Reference))
  (|CallParentFunction Character Type SubType bone Point Source)
  (bind _asmordhau_character (Utilities|Casting|CastToMordhauCharacter Character))
  (if (Utilities|Name|Equal(Name) bone "head")
    (Class|MordhauCharacter|QueueDismember _asmordhau_character (Variables|Default|GetNewVar_0) false true (Math|Vector|MakeVector 0.0 0.0 0.0) self)))

(event EventBeginPlay)

(event Collision|EventActorBeginOverlap
  (params (OtherActor :type Actor%20Object%20Reference)))

(event EventTick
  (params (DeltaSeconds :type Float%20%28single-precision%29)))

(event EventOnProjectileHitCosmetic
  (params (OtherActor :type Actor%20Object%20Reference) (Hit :type Hit%20Result%20Structure%20%28by%20ref%29))
  (|CallParentFunction OtherActor Hit)
  (bind _asmordhau_character (Utilities|Casting|CastToMordhauCharacter OtherActor))
  (if (stale _returnvalue)
    (if (Utilities|Name|Equal(Name) (.HitBoneName (Collision|BreakHitResult Hit)) "head")
      (Class|MordhauCharacter|QueueDismember _asmordhau_character (Variables|Default|GetNewVar_1) false true (Math|Vector|MakeVector 0.0 0.0 0.0) self))))

(event EventProcessProjectileHit
  (params (bIsBlocking :type Boolean) (Hit :type Hit%20Result%20Structure%20%28by%20ref%29))
  (Utilities|FlowControl|Sequence
    (:then_0
      (Variables|Default|SetDamageMultiplier (Math|Float|MapRangeClamped (.Z (Math|Vector|BreakVector (Transformation|GetVelocity))) -8e+02 -9e+02 0.1 1.0)))
    (:then_1
      (|CallParentFunction bIsBlocking Hit))))

(fn ConstructionScript
  (|CallParentFunction))