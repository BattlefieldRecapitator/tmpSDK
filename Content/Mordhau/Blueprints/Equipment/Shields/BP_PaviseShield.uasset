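; Deployable pavise shield equipment that a character plants as a damageable barrier, using the loaded state for carried versus planted.
; Firing needs a grounded user and a plane trace finding flat enough ground, then drops and attaches the shield, toggling blocker collision and parry mask.
; Only the planter can interact within an angle limit to unplant it; vehicle overlap also unplants.
; Accumulated damage zeroes ammo, ragdolling it; destruction or planter death starts a despawn timer.
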(event OnComponentBeginOverlap(MovementBlocker)
  (params (OverlappedComponent :type Primitive%20Component%20Object%20Reference) (OtherActor :type Actor%20Object%20Reference) (OtherComp :type Primitive%20Component%20Object%20Reference) (OtherBodyIndex :type Integer) (bFromSweep :type Boolean) (SweepResult :type Hit%20Result%20Structure%20%28by%20ref%29))
  (Networking|SwitchHasAuthority
    (:Authority
      (Utilities|Casting|CastToMordhauVehicle OtherActor)
      (if (not (Variables|Default|GetbIsLoaded))
        (Class|MordhauEquipment|SetLoaded true)))))

(event Custom|PlanterDied
  (params (Character :type Advanced%20Character%20Object%20Reference))
  (Networking|SwitchHasAuthority
    (:Authority
      (if (<= (Actor|GetLifeSpan) 0.0)
        (Actor|SetLifeSpan 1e+01)))))

(event Custom|PlanterDestroyed
  (params (Character :type Advanced%20Character%20Object%20Reference))
  (Networking|SwitchHasAuthority
    (:Authority
      (if (<= (Actor|GetLifeSpan) 0.0)
        (Actor|SetLifeSpan 1e+01)))))

(event EventOnHeldInteractionStart
  (params (Character :type Mordhau%20Character%20Object%20Reference))
  (if (Variables|Default|GetbIsLoaded)
    _
    (else
      (Class|MordhauEquipment|SetLoaded true)))
  (|CallParentFunction Character))

(event EventOnLoadedChanged
  (bind _movementblocker (Variables|Default|GetMovementBlocker))
  (bind _skeletalmeshcomponent (Variables|Default|GetSkeletalMeshComponent))
  (bind _plantercharacter (Variables|Default|GetPlanterCharacter))
  (|CallParentFunction)
  (if (!= (stale _returnvalue) 0)
    (Utilities|FlowControl|Sequence
      (:then_0
        (if (Variables|Default|GetbIsLoaded)
          (Networking|SwitchHasAuthority
            (:Authority
              (Transformation|DetachFromActor "KeepWorld" "KeepWorld" "KeepWorld"))
            (:Remote
              _))
          (Collision|SetCollisionEnabled _movementblocker "NoCollision")
          (Variables|/Script/Engine.PrimitiveComponent|SetbGenerateOverlapEvents _movementblocker false)
          (Components|Animation|PlayAnimation _skeletalmeshcomponent 0 false)
          (Variables|Default|SetbCanRagdoll true)
          (Variables|Default|SetParryMask (Variables|Default|GetParryMaskUnplanted))
          (Utilities|IsValid _plantercharacter
            (:Is%20Valid
              (EventDispatchers|UnbindEventfromOnCharacterDied _plantercharacter (delegate Custom|PlanterDied))
              (EventDispatchers|UnbindEventfromOnCharacterDestroyed _plantercharacter (delegate Custom|PlanterDestroyed))))
          (else
            (Variables|Default|SetReceivedDamage 0.0)
            (Variables|/Script/Engine.PrimitiveComponent|SetbGenerateOverlapEvents _movementblocker true)
            (Collision|SetCollisionEnabled _movementblocker "QueryAndPhysics")
            (Components|Animation|PlayAnimation _skeletalmeshcomponent 0 false)
            (Variables|Default|SetbCanRagdoll false)
            (Variables|Default|SetParryMask (Variables|Default|GetParryMaskPlanted)))))
      (:then_1
        (Class|MordhauEquipment|UpdateEquipmentState)))))

(event EventOnInteractionStart
  (params (Character :type Mordhau%20Character%20Object%20Reference))
  (if (Variables|Default|GetbIsLoaded)
    _
    (else
      (Class|MordhauEquipment|SetLoaded true)))
  (|CallParentFunction Character))

(event EventOnAmmoChanged
  (bind _skeletalmeshcomponent (Variables|Default|GetSkeletalMeshComponent))
  (bind _skeletalmeshcomponent_2 (Variables|Default|GetSkeletalMeshComponent))
  (bind _movementblocker (Variables|Default|GetMovementBlocker))
  (bind _destroysound (Variables|Default|GetDestroySound))
  (bind _returnvalue (Transformation|GetWorldLocation _skeletalmeshcomponent))
  (|CallParentFunction)
  (if (== (stale _returnvalue) 0)
    (Variables|Default|SetbIsInteractable false)
    (Utilities|FlowControl|Sequence
      (:then_0
        (Collision|SetCollisionEnabled (Variables|Default|GetProjectileBlock) "NoCollision")
        (Utilities|IsValid _movementblocker
          (:Is%20Valid
            (Collision|SetCollisionEnabled _movementblocker "NoCollision"))))
      (:then_1
        (Networking|CanExecuteCosmeticEvents
          (:True
            (Class|SkinnedMeshComponent|SetSkeletalMesh _skeletalmeshcomponent_2 "/Game/Mordhau/Assets/Weapons/Shields/Pavise/PaviseRagdoll.PaviseRagdoll" false)
            (Collision|SetCollisionProfileName _skeletalmeshcomponent_2 "IgnoringRagdoll" :!class /Script/Engine.PrimitiveComponent)
            (Physics|SetSimulatePhysics _skeletalmeshcomponent_2 true)
            (Physics|AddRadialForce _skeletalmeshcomponent _returnvalue 1e+02 1e+04 "RIF_Constant" true)
            (Utilities|IsValid _destroysound
              (:Is%20Valid
                (Audio|PlaySoundatLocation _destroysound _returnvalue "0, 0, 0" 1.0 1.0 0.0 0 0 0))))))
      (:then_2
        (Networking|SwitchHasAuthority
          (:Authority
            (Actor|SetLifeSpan 1e+01)))))))

(event EventFireProjectile
  (params (Origin :type Vector%20%28by%20ref%29 :default "0, 0, 0") (Orientation :type Rotator%20%28by%20ref%29 :default "0, 0, 0") (OwningController :type Controller%20Object%20Reference) (ExpectedDelay :type Float%20%28single-precision%29))
  (bind _returnvalue (Class|MordhauEquipment|GetParentCharacter))
  (Audio|SpawnSoundAttached (Variables|Default|GetFireSound) (Variables|Default|GetSkeletalMeshComponent) "None" "0, 0, 0" "0, 0, 0" "SnapToTarget" false 1.0 1.0 0.0 0 0)
  (Variables|Default|SetPlanterCharacter 0)
  (Variables|Default|SetPlanterController 0)
  (Utilities|IsValid _returnvalue
    (:Is%20Valid
      (bind _output_get (Variables|Default|SetPlanterCharacter _returnvalue))
      (Variables|Default|SetPlanterController (Pawn|GetController _output_get))
      (Networking|SwitchHasAuthority
        (:Authority
          (EventDispatchers|BindEventtoOnCharacterDied _output_get (delegate Custom|PlanterDied))
          (EventDispatchers|BindEventtoOnCharacterDestroyed _output_get (delegate Custom|PlanterDestroyed))
          (bind (_succeeded _location _rotation _attachtocomponent) (CallFunction|ValidatePlantSpot (Transformation|GetActorLocation _returnvalue) Orientation))
          (if _succeeded
            (Class|MordhauEquipment|SetLoaded false)
            (Class|MordhauCharacter|DropEquipment _returnvalue self)
            (Transformation|SetActorLocationAndRotation _location _rotation)
            (Transformation|AttachComponentToComponent _attachtocomponent "None" "KeepWorld" "KeepWorld" "KeepWorld" false)))))))

(event Game|Damage|EventAnyDamage
  (params (Damage :type Float%20%28single-precision%29) (DamageType :type Damage%20Type%20Object%20Reference) (InstigatedBy :type Controller%20Object%20Reference) (DamageCauser :type Actor%20Object%20Reference))
  (|CallParentFunction Damage DamageType InstigatedBy DamageCauser)
  (Networking|SwitchHasAuthority
    (:Authority
      (if (not (Variables|Default|GetbIsLoaded))
        (bind _asmordhau_character (Utilities|Casting|CastToMordhauCharacter DamageCauser)
          (:then
            (bind _asattack_motion (Utilities|Casting|CastToAttackMotion (Variables|/Script/Mordhau.MordhauCharacter|GetMotion _asmordhau_character))
              (:then
                (if (Utilities|Enum|Equal(Enum) (Variables|/Script/Mordhau.AttackMotion|GetMove _asattack_motion) "Kick")
                  (CallFunction|HandleTakeDamage 31.0)
                  (else
                    (CallFunction|HandleTakeDamage Damage :!label _label))))
              (:CastFailed
                (goto _label))))
          (:CastFailed
            (goto _label)))))))

(fn ConstructionScript
  (|CallParentFunction))

(fn ValidatePlantSpot
  (params (PlantLocation :type Vector) (CameraRotation1P :type Rotator))
  (bind _yaw (Math|Rotator|BreakRotator CameraRotation1P))
  (bind _returnvalue (Math|Rotator|MakeRotator 0.0 0.0 _yaw))
  (bind _returnvalue_2 (Math|Vector|GetForwardVector _returnvalue))
  (bind _returnvalue_3 (Math|Vector|GetRightVector _returnvalue))
  (bind _returnvalue_4 (* _returnvalue_2 1e+02))
  (bind _returnvalue_5 (+ PlantLocation _returnvalue_4))
  (bind (_lefthit _righthit _forwardhit _backhit _outright _outforward _returnvalue_6) (Class|MordhauUtilityLibrary|PlaneTrace (+ (* _returnvalue_3 -25.0) _returnvalue_5) (+ _returnvalue_5 (* _returnvalue_3 25.0)) _returnvalue_5 (+ PlantLocation (* _returnvalue_2 6e+01)) (Math|Vector|MakeVector 0.0 0.0 -1.5e+02) (Utilities|Array|MakeArray "ObjectTypeQuery1" "ObjectTypeQuery5") false (Utilities|Array|MakeArray 0) false true (Math|Vector|MakeVector 0.0 0.0 1e+01) false))
  (if _returnvalue_6
    (bind _output_get (LocalVariables|SetFoundRot (Math|Rotator|MakeRotfromXY (* _outforward -1.0) (* _outright -1.0))))
    (if (< (Class|KismetMathLibrary|DegAcos (Math|Vector|DotProduct (Math|Vector|GetUpVector _output_get) "0, 0,1.000000")) 2e+01)
      (return true (+ (.ImpactPoint (Collision|BreakHitResult _forwardhit)) (Math|Vector|RotateVector "0, 0,75.000000" (LocalVariables|GetFoundRot))) (Math|Rotator|CombineRotators "-12.000000, 0, 0" (LocalVariables|GetFoundRot)) (.HitComponent (Collision|BreakHitResult _forwardhit)))
      (else
        _)))
  (return false "0, 0, 0" "0, 0, 0" 0))

(fn ShouldShine
  (if (Variables|Default|GetbIsLoaded)
    (bind _returnvalue (|CallParentFunction))
    (return _returnvalue)
    (else
      (return false))))

(fn OnRequestFire
  (params (Character :type Mordhau%20Character%20Object%20Reference))
  (if (Variables|Default|GetbIsLoaded)
    (bind _returnvalue (Class|AdvancedCharacter|IsAirborne Character))
    (if _returnvalue
      _
      (else
        (bind _succeeded (CallFunction|ValidatePlantSpot (Transformation|GetActorLocation Character) (Variables|/Script/Mordhau.MordhauCharacter|GetCameraRotation1P Character)))
        (if _succeeded
          (bind _returnvalue_2 (|CallParentFunction Character))
          (return _returnvalue_2)
          (else
            _)))))
  (Variables|/Script/Mordhau.MordhauCharacter|SetbWantsFire Character false)
  (Class|MordhauCharacter|OnActionFailed Character (LocalVariables|GetNewLocalVar_0))
  (return false))

(fn CanInteract
  (params (Character :type Mordhau%20Character%20Object%20Reference))
  (Utilities|IsValid Character
    (:Is%20Valid
      (if (Variables|Default|GetbIsLoaded)
        _
        (elif (and (== (Pawn|GetController Character) (Variables|Default|GetPlanterController)) (<= (Class|KismetMathLibrary|DegAcos (Math|Vector2D|DotProduct(2D) (Math|Vector2D|Normalize2D (Math|Conversions|ToVector2D(Vector) (- (Transformation|GetActorLocation Character) (Transformation|GetActorLocation)))) (Math|Vector2D|Normalize2D (Math|Conversions|ToVector2D(Vector) (Transformation|GetActorForwardVector))))) 6e+01))
          _
          (else
            (return false)))))
    (:Is%20Not%20Valid
      _))
  (return (stale _returnvalue)))

(fn HandleTakeDamage
  (params (Damage :type Float%20%28single-precision%29))
  (bind _output_get (Variables|Default|SetReceivedDamage (Math|Float|Max(Float) (+ (Variables|Default|GetReceivedDamage) Damage) 0.0)))
  (if (>= _output_get (Variables|Default|GetDamageToDestroy))
    (Class|MordhauEquipment|SetAmmo)))

(fn CanHeldInteract
  (params (Character :type Mordhau%20Character%20Object%20Reference))
  (Utilities|IsValid Character
    (:Is%20Valid
      (if (Variables|Default|GetbIsLoaded)
        _
        (elif (and (== (Pawn|GetController Character) (Variables|Default|GetPlanterController)) (<= (Class|KismetMathLibrary|DegAcos (Math|Vector2D|DotProduct(2D) (Math|Vector2D|Normalize2D (Math|Conversions|ToVector2D(Vector) (- (Transformation|GetActorLocation Character) (Transformation|GetActorLocation)))) (Math|Vector2D|Normalize2D (Math|Conversions|ToVector2D(Vector) (Transformation|GetActorForwardVector))))) 6e+01))
          _
          (else
            (return false)))))
    (:Is%20Not%20Valid
      _))
  (return (stale _returnvalue)))