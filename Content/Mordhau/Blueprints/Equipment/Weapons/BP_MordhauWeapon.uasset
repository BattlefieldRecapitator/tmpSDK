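; BP_MordhauWeapon is a weapon Blueprint that adds a thrown-trail effect and supplies the clash collider.
; StartThrownTrail calls its parent, attaches the P_ThrownTrail emitter to the skeletal mesh at StickyPoint and begins trails from that single socket.
; StopThrownTrail calls its parent, ends the trails and clears the stored particle reference.
; The construction script assigns the Blueprint's ClashCapsuleBP to ClashCollider.
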(event EventStopThrownTrail
  (|CallParentFunction)
  (Utilities|IsValid (Variables|Default|GetThrownParticle)
    (:Is%20Valid
      (Effects|Particles|Trails|EndTrails (Variables|Default|GetThrownParticle))
      (Variables|Default|SetThrownParticle 0))))

(event Collision|EventActorBeginOverlap
  (params (OtherActor :type Actor%20Object%20Reference)))

(event EventTick
  (params (DeltaSeconds :type Float%20%28single-precision%29)))

(event EventStartThrownTrail
  (|CallParentFunction)
  (bind _returnvalue (Effects|SpawnEmitterAttached "/Game/Mordhau/Particles/Blood/P_ThrownTrail.P_ThrownTrail" (Variables|Default|GetSkeletalMeshComponent) "StickyPoint"))
  (bind _output_get (Variables|Default|SetThrownParticle _returnvalue))
  (Utilities|IsValid _output_get
    (:Is%20Valid
      (Effects|Particles|Trails|BeginTrails _output_get "StickyPoint" "StickyPoint" "ETrailWidthMode_FromCentre" 1.0))))

(fn ConstructionScript
  (Variables|Default|SetClashCollider (Variables|Default|GetClashCapsuleBP)))