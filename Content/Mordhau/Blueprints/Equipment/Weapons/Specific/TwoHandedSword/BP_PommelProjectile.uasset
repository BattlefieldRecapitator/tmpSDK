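; BP_PommelProjectile is the projectile for a two-handed sword's pommel, matching its mesh to the equipment that fired it.
; On firing, it runs the parent logic, casts the projectile creator to MordhauEquipment and searches its part instances.
; The first valid auxiliary skeletal mesh found becomes the projectile's skeletal mesh, so no per-pommel mesh is set in this Blueprint's graph.
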(event EventOnProjectileFired
  (|CallParentFunction)
  (bind _returnvalue (Class|MordhauProjectile|GetProjectileCreator))
  (bind _asmordhau_equipment (Utilities|Casting|CastToMordhauEquipment _returnvalue))
  (bind _array_element (Utilities|Array|ForEachLoopwithBreak (Variables|/Script/Mordhau.MordhauEquipment|GetPartInstances _asmordhau_equipment) :!label _label)
    (:LoopBody
      (Utilities|IsValid (Variables|/Script/Mordhau.MordhauEquipmentPart|GetAuxiliarySkeletalMesh _array_element)
        (:Is%20Valid
          (Class|SkinnedMeshComponent|SetSkeletalMesh (Variables|Default|GetSkeletalMeshComponent) (Variables|/Script/Mordhau.MordhauEquipmentPart|GetAuxiliarySkeletalMesh _array_element) true)
          (goto _label Break))))))

(event EventBeginPlay)

(event Collision|EventActorBeginOverlap
  (params (OtherActor :type Actor%20Object%20Reference)))

(event EventTick
  (params (DeltaSeconds :type Float%20%28single-precision%29)))

(fn ConstructionScript
  (|CallParentFunction))