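; BP_Bow is the bow ranged weapon Blueprint, adding a cosmetic link between its loaded state and its animation.
; It casts the skeletal mesh's anim instance to AB_Bow and sets LoadedIn1P as a float, nonzero only when loaded and the parent is in first person.
; This refresh runs after the parent logic on BeginPlay, on loaded changes, and on equipment visual updates when cosmetic events can execute.
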(event EventBeginPlay
  (|CallParentFunction)
  (bind _asab_bow (Utilities|Casting|CastToAB_Bow (Components|SkeletalMesh|GetAnimInstance (Variables|Default|GetSkeletalMeshComponent))))
  (Variables|/Game/Mordhau/Animations/Blueprints/AB_Bow.AB_Bow_C|SetLoadedIn1P _asab_bow (Math|Conversions|ToFloat(Boolean) (and (Variables|Default|GetbIsLoaded) (Variables|Default|GetbIsParentInFirstPerson)))))

(event EventActorBeginOverlap
  (params (OtherActor :type Actor%20Object%20Reference)))

(event EventTick
  (params (DeltaSeconds :type Float%20%28single-precision%29)))

(event EventUpdateEquipmentVisualState
  (|CallParentFunction)
  (Networking|CanExecuteCosmeticEvents
    (:True
      (bind _asab_bow (Utilities|Casting|CastToAB_Bow (Components|SkeletalMesh|GetAnimInstance (Variables|Default|GetSkeletalMeshComponent))))
      (Variables|/Game/Mordhau/Animations/Blueprints/AB_Bow.AB_Bow_C|SetLoadedIn1P _asab_bow (Math|Conversions|ToFloat(Boolean) (and (Variables|Default|GetbIsLoaded) (Variables|Default|GetbIsParentInFirstPerson)))))))

(event EventOnLoadedChanged
  (|CallParentFunction)
  (bind _asab_bow (Utilities|Casting|CastToAB_Bow (Components|SkeletalMesh|GetAnimInstance (Variables|Default|GetSkeletalMeshComponent))))
  (Variables|/Game/Mordhau/Animations/Blueprints/AB_Bow.AB_Bow_C|SetLoadedIn1P _asab_bow (Math|Conversions|ToFloat(Boolean) (and (Variables|Default|GetbIsLoaded) (Variables|Default|GetbIsParentInFirstPerson)))))

(fn ConstructionScript
  (|CallParentFunction))