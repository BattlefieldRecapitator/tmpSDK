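; Crossbow ranged weapon Blueprint that keeps its visuals in sync with whether it is loaded.
; On begin play and whenever the loaded state changes, it writes that state as a float into the Loaded variable of its Crossbow_AB animation instance.
; The construction script snaps the Missile component onto the skeletal mesh's BoltSocket.
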(event EventBeginPlay
  (|CallParentFunction)
  (bind _ascrossbow_ab (Utilities|Casting|CastToCrossbow_AB (Components|SkeletalMesh|GetAnimInstance (Variables|Default|GetMesh))))
  (Variables|/Game/Mordhau/Assets/Weapons/Crossbow/Crossbow_AB.Crossbow_AB_C|SetLoaded _ascrossbow_ab (Math|Conversions|ToFloat(Boolean) (Variables|Default|GetbIsLoaded))))

(event EventActorBeginOverlap
  (params (OtherActor :type Actor%20Object%20Reference)))

(event EventTick
  (params (DeltaSeconds :type Float%20%28single-precision%29)))

(event EventOnLoadedChanged
  (|CallParentFunction)
  (bind _ascrossbow_ab (Utilities|Casting|CastToCrossbow_AB (Components|SkeletalMesh|GetAnimInstance (Variables|Default|GetMesh))))
  (Variables|/Game/Mordhau/Assets/Weapons/Crossbow/Crossbow_AB.Crossbow_AB_C|SetLoaded _ascrossbow_ab (Math|Conversions|ToFloat(Boolean) (Variables|Default|GetbIsLoaded))))

(fn ConstructionScript
  (|CallParentFunction)
  (Transformation|AttachComponentToComponent (Variables|Default|GetMissile) (Variables|Default|GetSkeletalMeshComponent) "BoltSocket" "SnapToTarget" "SnapToTarget" "SnapToTarget" true))