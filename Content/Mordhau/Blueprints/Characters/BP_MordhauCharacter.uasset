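; Placeholder Mordhau player character with basic look, movement, jump, Shift sprint and a fake interact on E.
; A one-second timer counts how long E is held; on release, a debug-drawn camera trace calls held or normal interaction on a MordhauActor.
; An AdvancedCharacter hit receives only the normal interaction.
; A looping timer feeds camera pitch into the animation Blueprint's head rotation.
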(event Custom|CountTimeEHeld
  ;[1 1 1] FakeInteract
  (Math|Integer|IncrementInt (stale Input|KeyboardEvents|E _output_get)))

(event EventBeginPlay
  (Utilities|Time|SetTimerbyFunctionName 0 "UpdateHead" 0.1 true)
  (bind _output_get (Variables|Default|SetWalkSpeed (Variables|/Script/Engine.CharacterMovementComponent|GetMaxWalkSpeed (Variables|Character|GetCharacterMovement))))
  (Variables|Default|SetRunSpeed (+ _output_get 2e+02)))

(event Collision|EventActorBeginOverlap
  (params (OtherActor :type Actor%20Object%20Reference)))

(event EventTick
  (params (DeltaSeconds :type Float%20%28single-precision%29))
  ;[1 1 1] FakeInteract
)

(event EventOnInteractionStart
  (params (Character :type Advanced%20Character%20Object%20Reference))
  (bind _returnvalue (Game|GetPlayerCameraManager 0))
  (bind _self self)
  (bind _returnvalue_2 (Transformation|GetActorLocation _returnvalue))
  ;[1 1 1] FakeInteract
  (bind _outhit (Collision|LineTraceForObjects _returnvalue_2 (+ (* (Transformation|GetActorForwardVector _returnvalue) 5e+03) _returnvalue_2) (Utilities|Array|MakeArray "ObjectTypeQuery1" "ObjectTypeQuery2" "ObjectTypeQuery3") false 0 "ForDuration" true "(R=1.000000,G=0.000000,B=0.000000,A=1.000000)" "(R=0.000000,G=1.000000,B=0.000000,A=1.000000)" 3.0))
  (bind _asmordhau_actor (Utilities|Casting|CastToMordhauActor (.HitActor (Collision|BreakHitResult _outhit)))
    (:then
      (if (Variables|Default|GetHeld)
        (Class|MordhauActor|OnHeldInteractionStart _asmordhau_actor _self)
        (Development|PrintString (Utilities|String|Append "Held Interacted With:" (Utilities|GetDisplayName _asmordhau_actor)))
        (else
          (Class|MordhauActor|OnInteractionStart _asmordhau_actor _self)
          (Development|PrintString (Utilities|String|Append "Interacted With:" (Utilities|GetDisplayName _asmordhau_actor))))))
    (:CastFailed
      (bind _asadvanced_character (Utilities|Casting|CastToAdvancedCharacter (.HitActor (Collision|BreakHitResult _outhit))))
      (Class|AdvancedCharacter|OnInteractionStart _asadvanced_character _self))))

(event Input|AxisEvents|InputAxisTurn
  (params (AxisValue :type Float%20%28single-precision%29))
  ;[1 1 1] Placeheld By TheMattman
  (Pawn|Input|AddControllerYawInput (Pawn|GetControlledPawn (Pawn|GetController)) AxisValue))

(event Input|AxisEvents|InputAxisLookUp
  (params (AxisValue :type Float%20%28single-precision%29))
  ;[1 1 1] Placeheld By TheMattman
  (Pawn|Input|AddControllerPitchInput (Pawn|GetControlledPawn (Pawn|GetController)) AxisValue))

(event Input|AxisEvents|InputAxisMoveForward
  (params (AxisValue :type Float%20%28single-precision%29))
  ;[1 1 1] Placeheld By TheMattman
  (Pawn|Input|AddMovementInput (Math|Vector|GetForwardVector (Math|Rotator|MakeRotator 0.0 0.0 (.Yaw (Math|Rotator|BreakRotator (Pawn|GetControlRotation :!class /Script/Engine.Pawn))))) AxisValue false))

(event Input|AxisEvents|InputAxisMoveRight
  (params (AxisValue :type Float%20%28single-precision%29))
  ;[1 1 1] Placeheld By TheMattman
  (Pawn|Input|AddMovementInput (Math|Vector|GetRightVector (Math|Rotator|MakeRotator 0.0 0.0 (.Yaw (Math|Rotator|BreakRotator (Pawn|GetControlRotation :!class /Script/Engine.Pawn))))) AxisValue false))

(event Input|KeyboardEvents|SpaceBar
  (params (Key :type Key%20Structure))
  ;[1 1 1] Placeheld By TheMattman
  (:Pressed
    (Character|Jump)))

(event Input|KeyboardEvents|E
  (params (Key :type Key%20Structure))
  ;[1 1 1] FakeInteract
  (:Pressed
    (bind _output_get (Variables|Default|SetHeldE 0))
    (bind _returnvalue (Utilities|Time|SetTimerbyEvent (delegate Custom|CountTimeEHeld) 1.0 true)))
  (:Released
    (Utilities|Time|ClearandInvalidateTimerbyHandle _returnvalue)
    (if (> (Variables|Default|GetHeldE) 1)
      (Variables|Default|SetHeld true)
      (else
        (Variables|Default|SetHeld false)))
    (Class|AdvancedCharacter|OnInteractionStart self)))

(event Input|KeyboardEvents|LeftShift
  (params (Key :type Key%20Structure))
  (bind _charactermovement (Variables|Character|GetCharacterMovement))
  (:Pressed
    (Variables|/Script/Engine.CharacterMovementComponent|SetMaxWalkSpeed _charactermovement (Variables|Default|GetRunSpeed)))
  (:Released
    (Variables|/Script/Engine.CharacterMovementComponent|SetMaxWalkSpeed _charactermovement (Variables|Default|GetWalkSpeed))))

(fn ConstructionScript)

(fn UpdateHead
  (bind _asab_mordhau_character_animation (Utilities|Casting|CastToAB_MordhauCharacterAnimation (Components|SkeletalMesh|GetAnimInstance (Variables|Character|GetMesh))))
  (Variables|/Game/Mordhau/Animations/Blueprints/AB_MordhauCharacterAnimation.AB_MordhauCharacterAnimation_C|SetHeadRotation _asab_mordhau_character_animation (Math|Rotator|MakeRotator (+ (* (.pitch (Transformation|GetWorldRotation (Variables|Default|GetCamera))) -1.0) 9e+01) 0.0 0.0)))