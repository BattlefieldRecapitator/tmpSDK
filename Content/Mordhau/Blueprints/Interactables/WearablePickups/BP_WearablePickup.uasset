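; Base wearable pickup that a Battle Royale character interacts with to equip armor.
; On interaction it finds every ArmorInstance actor and, for each, updates the character's profile, calls Equip and posts a debug-like "2Assignment" message to the HUD chatbox.
; Equip, EquipIfUpgrade, IsAnUpgrade and AssignToCharacter are empty here, and the AssignToCharacter call is disconnected.
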(event EventBeginPlay)

(event Collision|EventActorBeginOverlap
  (params (OtherActor :type Actor%20Object%20Reference)))

(event EventTick
  (params (DeltaSeconds :type Float%20%28single-precision%29)))

(event EventOnInteractionStart
  (params (Character :type Mordhau%20Character%20Object%20Reference))
  (bind _asbp_battle_royale_character (Utilities|Casting|CastToBP_BattleRoyaleCharacter Character))
  (bind _outactors (Actor|GetAllActorsOfClass "/Game/Mordhau/Maps/NewTest/ArmorInstance.ArmorInstance_C"))
  (for _array_element _outactors
    (Class|CustomizationReplicationActor|UpdateCharacterProfile _array_element Character)
    (CallFunction|Equip _asbp_battle_royale_character)
    (bind _asplayer_controller (Utilities|Casting|CastToPlayerController (Pawn|GetController Character)))
    (bind _asbp_mordhau_hud (Utilities|Casting|CastToBP_MordhauHUD (HUD|GetHUD _asplayer_controller)))
    (Default|SendMessagetoChatbox _asbp_mordhau_hud "" "2Assignment")))

(fn ConstructionScript)

(fn EquipifUpgrade
  (params (Char :type Mordhau%20Character%20Object%20Reference)))

(fn Equip
  (params (Char :type Mordhau%20Character%20Object%20Reference)))

(fn IsAnUpgrade
  (params (Char :type BP%20Battle%20Royale%20Character%20Object%20Reference) (Value :type Boolean)))

(fn AssigntoCharacter
  (params (Character :type Mordhau%20Character%20Object%20Reference) (CustomizationReplicationActor :type Customization%20Replication%20Actor%20Object%20Reference)))