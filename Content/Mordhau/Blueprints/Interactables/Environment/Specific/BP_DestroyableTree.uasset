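; Destructible tree interactable that topples with effects when its replicated health reaches zero.
; The health update reveals the log, records the fall start and enables Tick, which blends the log toward the PreviewTree transform along a bounce curve, then disables itself.
; A delayed impact plays particles, sound and camera shake.
; Radial crush damage nodes are unconnected, so the recorded last-hit instigator goes unused.
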(event Collision|EventActorBeginOverlap
  (params (OtherActor :type Actor%20Object%20Reference))
  (|CallParentFunction OtherActor) ; This node is disabled and will not be called.\nDrag off pins to build functionality.
)

(event EventTick
  (params (DeltaSeconds :type Float%20%28single-precision%29))
  (bind _returnvalue (Utilities|Time|GetTimeSeconds))
  (bind _fallstarttime (Variables|Default|GetFallStartTime))
  (bind _returnvalue_2 (+ _fallstarttime 5.0))
  (bind _returnvalue_3 (Class|MordhauUtilityLibrary|GetNormalizedTime _fallstarttime _returnvalue_2 _returnvalue))
  (|CallParentFunction DeltaSeconds)
  (if (not (== (Variables|Default|GetFallStartTime) -1.0))
    (Transformation|SetRelativeTransform (Variables|Default|GetBreakableTree_Log) (Math|Transform|Lerp(Transform) (Variables|Default|GetFallingLogOrigin) (Transformation|GetRelativeTransform (Variables|Default|GetPreviewTree)) (Math|Curves|GetFloatValue (Variables|Default|GetBounceCurve) _returnvalue_3)) false false)
    (if (== _returnvalue_3 1.0)
      (Actor|Tick|SetActorTickEnabled false))))

(event EventUpdateReplicatedHealth
  (bind _breakabletree_log (Variables|Default|GetBreakableTree_Log))
  (bind _impact3 (Variables|Default|GetImpact3))
  (bind _returnvalue (Transformation|GetWorldLocation _impact3))
  (bind _returnvalue_2 (Transformation|GetWorldLocation _breakabletree_log))
  (|CallParentFunction)
  (Variables|Default|SetFinalChopperController (Variables|Default|GetLastHealthChangeInstigator))
  (if (== (Variables|Default|GetReplicatedHealth) 0)
    (if (== (Variables|Default|GetFallStartTime) -1.0)
      (Variables|Default|SetFallingLogOrigin (Transformation|GetRelativeTransform (Variables|Default|GetBreakableTree_Log)))
      (Variables|Default|SetFallStartTime (Utilities|Time|GetTimeSeconds))
      (Actor|Tick|SetActorTickEnabled true)
      (Development|SetHiddeninGame (Variables|Default|GetBreakableTree_Log) false false)
      (Audio|PlaySoundatLocation 0 _returnvalue_2 "0, 0, 0" 1.0 1.0 0.0 0 0 0)
      (Effects|SpawnEmitteratLocation 0 _returnvalue_2)
      (Utilities|FlowControl|Delay 3.3)
      (Effects|SpawnEmitteratLocation 0 _returnvalue "90.000000, 0,0.000000")
      (Audio|PlaySoundatLocation 0 _returnvalue "0, 0, 0" 1.0 1.0 0.0 0 0 0)
      (Camera|PlayWorldCameraShake 0 (Transformation|GetWorldLocation (Variables|Default|GetImpact2)) 2.5e+02 7.5e+03 1e+01))))

(fn ConstructionScript
  (|CallParentFunction))