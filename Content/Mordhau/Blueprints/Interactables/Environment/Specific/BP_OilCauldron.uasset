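; Interactable oil cauldron that pours oil and spawns a fire field, then reloads before it can be used again.
; Interaction by a player-controlled character stores that controller and sets State, whose OnRep drives idle, pour and recover phases and allows interaction only when idle.
; Each phase handles its animation, with effects, sounds and delays for pour and recover, while only the authority advances State afterward.
; The fire field records the last user as instigator.
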(event Custom|ReleaseOil
  (bind _oil (Variables|Default|GetOil))
  (Components|Animation|PlayAnimation (Variables|Default|GetSkeletalMeshComponent) 0 false)
  (Components|Activation|Activate _oil false)
  (Audio|Components|Audio|Play (Variables|Default|GetSC_CauldronPour) 0.0)
  (Utilities|FlowControl|Delay (Variables|Default|GetSpawnFireTime))
  (bind _returnvalue (Game|SpawnActorfromClass "/Game/Mordhau/Blueprints/Fields/BP_FireField.BP_FireField_C" (Transformation|GetWorldTransform (Variables|Default|GetFire)) "Undefined" 0 0))
  (Variables|/Game/Mordhau/Blueprints/Fields/BP_MasterField.BP_MasterField_C|SetInstigatorController _returnvalue (Variables|Default|GetLastUserController))
  (Audio|Components|Audio|Play (Variables|Default|GetCauldronSplash) 0.0)
  (Components|Activation|Deactivate _oil)
  (Networking|SwitchHasAuthority
    (:Authority
      (Variables|Default|SetState 2))))

(event Custom|Recover
  (bind _skeletalmeshcomponent (Variables|Default|GetSkeletalMeshComponent))
  (bind _reloadtime (Variables|Default|GetReloadTime))
  (Components|Animation|PlayAnimation _skeletalmeshcomponent 0 false)
  (Components|Timeline|SetPlayRate _skeletalmeshcomponent (/ 1.0 _reloadtime))
  (Utilities|FlowControl|Delay _reloadtime)
  (Audio|Components|Audio|Play (Variables|Default|GetCauldronReload) 0.0)
  (Networking|SwitchHasAuthority
    (:Authority
      (Variables|Default|SetState 0))))

(event Custom|Idle
  (Components|Animation|SetAnimation (Variables|Default|GetSkeletalMeshComponent) 0))

(event EventBeginPlay
  (|CallParentFunction) ; This node is disabled and will not be called.\nDrag off pins to build functionality.
)

(event Collision|EventActorBeginOverlap
  (params (OtherActor :type Actor%20Object%20Reference))
  (|CallParentFunction OtherActor) ; This node is disabled and will not be called.\nDrag off pins to build functionality.
)

(event EventTick
  (params (DeltaSeconds :type Float%20%28single-precision%29))
  (|CallParentFunction DeltaSeconds) ; This node is disabled and will not be called.\nDrag off pins to build functionality.
)

(event EventOnInteractionStart
  (params (Character :type Mordhau%20Character%20Object%20Reference))
  (Utilities|IsValid Character
    (:Is%20Valid
      (bind _asplayer_controller (Utilities|Casting|CastToPlayerController (Pawn|GetController Character)))
      (Variables|Default|SetLastUserController _asplayer_controller)
      (Variables|Default|SetState 1))))

(fn ConstructionScript
  (|CallParentFunction))

(fn OnRepState
  (bind _state (Variables|Default|GetState))
  (if (== _state 0)
    (Variables|Default|SetbIsInteractable true)
    (CallFunction|Idle)
    (else
      (Variables|Default|SetbIsInteractable false)
      (if (== _state 1)
        (CallFunction|ReleaseOil)
        (elif (== _state 2)
          (CallFunction|Recover))))))