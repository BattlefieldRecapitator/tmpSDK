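; Ammo box interactable that restocks a character's equipment when used.
; Restock checks the player controller's cooldown time, tops up ammo by each item's restock amount, restocks default equipment, then increments a replicated cooldown counter if anything changed.
; Interaction and widget visibility depend on the depleted state and the local controller's IsAnythingRestockable flag.
; Deplete and Refill hackily override local chest behavior, since availability is global per player.
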(event Custom|Refill
  ;[1 1 1] This is a hack to override local chest functionality. Ammo boxes do this directly in playercontroller, because they're global per player
  (Variables|Default|SetIsDepleted false)
  (CallFunction|Refilled))

(event EventDeplete
  (params (PlayerState :type Player%20State%20Object%20Reference))
  ;[1 1 1] This is a hack to override local chest functionality. Ammo boxes do this directly in playercontroller, because they're global per player
  (Variables|Default|SetIsDepleted true)
  (CallFunction|Depleted))

(event EventActorBeginOverlap
  (params (OtherActor :type Actor%20Object%20Reference)))

(event EventTick
  (params (DeltaSeconds :type Float%20%28single-precision%29)))

(event EventAvailableInteractionStart
  (params (Character :type Mordhau%20Character%20Object%20Reference))
  (CallFunction|Restock Character))

(fn ConstructionScript
  (|CallParentFunction))

(fn Restock
  (params (Character :type Mordhau%20Character%20Object%20Reference))
  (bind _returnvalue (Class|MordhauCharacter|GetControllerIncludingVehicle Character))
  (bind _asbp_mordhau_player_controller (Utilities|Casting|CastToBP_MordhauPlayerController _returnvalue))
  (if (< (Variables|/Game/Mordhau/Blueprints/BP_MordhauPlayerController.BP_MordhauPlayerController_C|GetNextAmmoBoxAvailableTime _asbp_mordhau_player_controller) (Utilities|Time|GetTimeSeconds))
    (Utilities|FlowControl|Sequence
      (:then_0
        (for _array_element (Variables|/Script/Mordhau.MordhauCharacter|GetEquipment Character)
          (Utilities|IsValid _array_element
            (:Is%20Valid
              (if (< (Class|MordhauEquipment|GetAmmo _array_element) (Class|MordhauEquipment|GetCurrentMaxAmmo _array_element))
                (Class|MordhauEquipment|SetAmmo _array_element (Math|Conversions|ToByte(Integer) (Math|Integer|Min(Integer) (+ (Math|Conversions|ToInteger(Byte) (Class|MordhauEquipment|GetAmmo _array_element)) (Variables|/Script/Mordhau.MordhauEquipment|GetMaxAmmoBoxRestockAmount _array_element)) (Math|Conversions|ToInteger(Byte) (Class|MordhauEquipment|GetCurrentMaxAmmo _array_element)))))
                (LocalVariables|SetRestocked true))))))
      (:then_1
        (bind _returnvalue_2 (Class|MordhauCharacter|RestockDefaultEquipment Character))
        (for _array_element_2 _returnvalue_2
          (Class|MordhauEquipment|SetAmmo _array_element_2 (Class|KismetMathLibrary|BMin (Class|MordhauEquipment|GetCurrentMaxAmmo _array_element_2) (Math|Conversions|ToByte(Integer) (Variables|/Script/Mordhau.MordhauEquipment|GetMaxAmmoBoxRestockAmount _array_element_2))))
          (LocalVariables|SetRestocked true)))
      (:then_2
        (if (LocalVariables|GetRestocked)
          (Variables|/Game/Mordhau/Blueprints/BP_MordhauPlayerController.BP_MordhauPlayerController_C|SetReplicatedAmmoBoxCooldown _asbp_mordhau_player_controller (+ (Variables|/Game/Mordhau/Blueprints/BP_MordhauPlayerController.BP_MordhauPlayerController_C|GetReplicatedAmmoBoxCooldown _asbp_mordhau_player_controller) 1)))))))

(fn CanInteract
  (params (Character :type Mordhau%20Character%20Object%20Reference))
  (if (Variables|Default|GetIsDepleted)
    _
    (else
      (bind _asmordhau_player_controller (Utilities|Casting|CastToMordhauPlayerController (Game|GetPlayerController 0))
        (:then
          (if (Pawn|IsLocalPlayerController _asmordhau_player_controller)
            (if (Variables|/Script/Mordhau.MordhauPlayerController|GetbIsAnythingRestockable _asmordhau_player_controller)
              (return (stale _returnvalue))
              (else
                _))
            (else
              (return (stale _returnvalue)))))
        (:CastFailed
          (return (stale _returnvalue))))))
  (return false))

(fn UpdateWidgetVisibilityOverride
  (bind _mordhauwidget (Variables|Default|GetMordhauWidget))
  (bind _asbp_mordhau_player_controller (Utilities|Casting|CastToBP_MordhauPlayerController (Game|GetPlayerController 0))
    (:then
      (if (and (Variables|/Script/Mordhau.MordhauPlayerController|GetbIsAnythingRestockable _asbp_mordhau_player_controller) (not (Variables|Default|GetIsDepleted)))
        (Variables|/Script/Mordhau.MordhauWidgetComponent|SetOverrideVisible _mordhauwidget -1)
        (else
          (Variables|/Script/Mordhau.MordhauWidgetComponent|SetOverrideVisible _mordhauwidget 0 :!label _label))))
    (:CastFailed
      (goto _label))))