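; Base actor for environment interactables driven by a progress value, with child classes expected to implement the empty ProgressUpdated hook.
; ProgressUpdatedInternal ignores unchanged values, remaps progress through optional separate raise or lower curves by direction, then passes it to that hook.
; On cosmetic-capable instances, after a brief startup delay and if audio is idle, it plays StartSound or EndSound when progress crosses their thresholds downward or upward respectively.
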(event EventBeginPlay)

(event Collision|EventActorBeginOverlap
  (params (OtherActor :type Actor%20Object%20Reference)))

(event EventTick
  (params (DeltaSeconds :type Float%20%28single-precision%29)))

(fn ConstructionScript)

(fn ProgressUpdated
  (params (Progress :type Float%20%28single-precision%29)))

(fn ProgressUpdatedInternal
  (params (Progress :type Float%20%28single-precision%29))
  (bind _audio (Variables|Default|GetAudio))
  (bind _progresscurveraise (Variables|Default|GetProgressCurveRaise))
  (bind _progresscurvelower (Variables|Default|GetProgressCurveLower))
  (bind _endsoundtriggertime (Variables|Default|GetEndSoundTriggerTime))
  (bind _audio_2 (Variables|Default|GetAudio))
  (if (not (Math|Float|NearlyEqual(Float) Progress (Variables|Default|GetLastProgress) 1e-06))
    (Utilities|FlowControl|Sequence
      (:then_0
        (Networking|CanExecuteCosmeticEvents
          (:True
            (if (and (>= (Utilities|Time|GetRealTimeSeconds) 2.0) (not (Audio|Components|Audio|IsPlaying (Variables|Default|GetAudio))))
              (Utilities|FlowControl|Sequence
                (:then_0
                  (Utilities|IsValid (Variables|Default|GetStartSound)
                    (:Is%20Valid
                      (if (and (> (Variables|Default|GetLastProgress) (Variables|Default|GetStartSoundTriggerTime)) (<= Progress (Variables|Default|GetStartSoundTriggerTime)))
                        (Audio|Components|Audio|SetSound _audio (Variables|Default|GetStartSound))
                        (Audio|Components|Audio|Play _audio 0.0)))))
                (:then_1
                  (Utilities|IsValid (Variables|Default|GetEndSound)
                    (:Is%20Valid
                      (if (and (< (Variables|Default|GetLastProgress) _endsoundtriggertime) (>= Progress _endsoundtriggertime))
                        (Audio|Components|Audio|SetSound _audio_2 (Variables|Default|GetEndSound))
                        (Audio|Components|Audio|Play _audio_2 0.0))))))))))
      (:then_1
        (if (>= Progress (Variables|Default|GetLastProgress))
          (Utilities|IsValid _progresscurveraise
            (:Is%20Valid
              (CallFunction|ProgressUpdated (Math|Curves|GetFloatValue _progresscurveraise Progress)))
            (:Is%20Not%20Valid
              (CallFunction|ProgressUpdated Progress :!label _label)))
          (else
            (Utilities|IsValid _progresscurvelower
              (:Is%20Valid
                (CallFunction|ProgressUpdated (Math|Curves|GetFloatValue _progresscurvelower Progress)))
              (:Is%20Not%20Valid
                (goto _label))))))
      (:then_2
        (Variables|Default|SetLastProgress Progress)))))