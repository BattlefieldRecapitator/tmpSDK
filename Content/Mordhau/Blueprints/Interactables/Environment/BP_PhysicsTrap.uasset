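; Interactable physics trap that releases its static mesh into physics simulation when used, or when damaged if damage activation is enabled.
; TriggerTrap records the instigating controller, sets Activated and starts a limited lifespan.
; The Activated RepNotify disables further interaction and enables physics on the server only.
; The trap can optionally destroy itself on mesh hit, and character overlap only prints a debug string.
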(event OnComponentHit(StaticMeshComponent)
  (params (HitComponent :type Primitive%20Component%20Object%20Reference) (OtherActor :type Actor%20Object%20Reference) (OtherComp :type Primitive%20Component%20Object%20Reference) (NormalImpulse :type Vector :default "0, 0, 0") (Hit :type Hit%20Result%20Structure%20%28by%20ref%29))
  (if (Variables|Default|GetDestroyOnImpact)
    (Actor|DestroyActor)))

(event EventBeginPlay)

(event EventTick
  (params (DeltaSeconds :type Float%20%28single-precision%29)))

(event EventOnInteractionStart
  (params (Character :type Mordhau%20Character%20Object%20Reference))
  (CallFunction|TriggerTrap (Pawn|GetController Character)))

(event Collision|EventActorBeginOverlap
  (params (OtherActor :type Actor%20Object%20Reference))
  (Utilities|Casting|CastToMordhauCharacter OtherActor)
  (Development|PrintString "Hello"))

(event Game|Damage|EventAnyDamage
  (params (Damage :type Float%20%28single-precision%29) (DamageType :type Damage%20Type%20Object%20Reference) (InstigatedBy :type Controller%20Object%20Reference) (DamageCauser :type Actor%20Object%20Reference))
  (if (and (Variables|Default|GetActivateOnDamage) (not (Variables|Default|GetActivated)))
    (CallFunction|TriggerTrap InstigatedBy)))

(fn ConstructionScript)

(fn OnRepActivated
  (bind _activated (Variables|Default|GetActivated))
  (Variables|Default|SetbIsInteractable (not _activated))
  (Networking|SwitchHasAuthority
    (:Authority
      (Physics|SetSimulatePhysics (Variables|Default|GetStaticMeshComponent) _activated))))

(fn TriggerTrap
  (params (InInstigatorController :type Controller%20Object%20Reference))
  (Variables|Default|SetInstigatorController InInstigatorController)
  (Variables|Default|SetActivated true)
  (Actor|SetLifeSpan (Variables|Default|GetLifeSpanWhenActivated)))