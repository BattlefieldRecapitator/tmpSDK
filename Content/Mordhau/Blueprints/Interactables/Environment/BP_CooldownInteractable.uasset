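; Base interactable Blueprint that becomes unavailable for a refill period after being depleted.
; Interaction start routes to an available or not-available event based on IsDepleted.
; Deplete disables interaction and sets IsDepleted, then restores both after RefillDelay.
; The IsDepleted RepNotify fires Depleted or Refilled, which are empty hooks here, as are both interaction events.
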(event Custom|Deplete
  (Variables|Default|SetbIsInteractable false)
  (Variables|Default|SetIsDepleted true)
  (Utilities|FlowControl|Delay (Variables|Default|GetRefillDelay))
  (Variables|Default|SetbIsInteractable true)
  (Variables|Default|SetIsDepleted false))

(event Custom|NotAvailableInteractionStart
  (params (Character :type Mordhau%20Character%20Object%20Reference)))

(event Custom|AvailableInteractionStart
  (params (Character :type Mordhau%20Character%20Object%20Reference)))

(event Custom|Refilled)

(event Custom|Depleted)

(event EventBeginPlay)

(event Collision|EventActorBeginOverlap
  (params (OtherActor :type Actor%20Object%20Reference)))

(event EventTick
  (params (DeltaSeconds :type Float%20%28single-precision%29)))

(event EventOnInteractionStart
  (params (Character :type Mordhau%20Character%20Object%20Reference))
  (if (Variables|Default|GetIsDepleted)
    (CallFunction|NotAvailableInteractionStart Character)
    (else
      (CallFunction|AvailableInteractionStart Character))))

(fn ConstructionScript
  (|CallParentFunction))

(fn OnRepIsDepleted
  (if (Variables|Default|GetIsDepleted)
    (CallFunction|Depleted)
    (else
      (CallFunction|Refilled))))