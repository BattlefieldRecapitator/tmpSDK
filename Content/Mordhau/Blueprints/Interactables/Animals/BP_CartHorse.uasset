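; BP_CartHorse is a horse Blueprint that, going by its name and mesh logic, is a cart-pulling variant.
; The construction script registers Capsule as the HorseMovementComponent's secondary and step-capable collision component.
; BeginPlay and BPLODTick only call their parents.
; Disconnected, never-run logic would aim StaticMesh at the Seat socket, spin Scene with horse movement and widen the anim instance's leg distance.
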(event EventBeginPlay
  (|CallParentFunction))

(event Collision|EventActorBeginOverlap
  (params (OtherActor :type Actor%20Object%20Reference)))

(event EventTick
  (params (DeltaSeconds :type Float%20%28single-precision%29)))

(event EventBPLODTick
  (params (DeltaTime :type Float%20%28single-precision%29))
  (|CallParentFunction DeltaTime))

(fn ConstructionScript
  (bind _capsule (Variables|Default|GetCapsule))
  (|CallParentFunction)
  (bind _ashorse_movement_component (Utilities|Casting|CastToHorseMovementComponent (Variables|Character|GetCharacterMovement)))
  (Variables|/Script/Mordhau.PseudoVehicleMovementComponent|SetSecondaryComponents _ashorse_movement_component (Utilities|Array|MakeArray _capsule))
  (Variables|/Script/Mordhau.PseudoVehicleMovementComponent|SetSecondaryStepCapableComponents _ashorse_movement_component (Utilities|Array|MakeArray _capsule)))