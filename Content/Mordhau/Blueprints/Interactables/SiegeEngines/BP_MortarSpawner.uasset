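; BP_MortarSpawner is a server-authoritative spawner that places a BP_Mortar at its capsule and respawns it after it dies.
; Spawning retries on a delay while the capsule overlaps anything, then applies optional look-up and turn limit overrides to the new mortar.
; Respawn timing reuses the game mode's ballista respawn time; on death, the wreck's lifespan is clamped to that time before the replacement spawns.
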(event Custom|OnBallistaDied
  (params (Character :type Advanced%20Character%20Object%20Reference))
  (Actor|SetLifeSpan Character (Math|Float|Clamp(Float) (Actor|GetLifeSpan Character) 0.01 (Variables|Default|GetRespawnTime))) ; Make sure the old ballista is removed before the new one spawns
  (Utilities|FlowControl|Delay (Variables|Default|GetRespawnTime))
  (CallFunction|Spawn))

(event Custom|Spawn
  (bind _overridelookuplimit (Variables|Default|GetOverrideLookUpLimit))
  (bind _overrideturnlimit (Variables|Default|GetOverrideTurnLimit))
  (bind _capsule (Variables|Default|GetCapsule))
  (Networking|SwitchHasAuthority
    (:Authority
      (bind _returnvalue (Collision|CapsuleOverlapActors (Transformation|GetWorldLocation _capsule) (Class|CapsuleComponent|GetUnscaledCapsuleRadius _capsule) (Components|Capsule|GetUnscaledCapsuleHalfHeight _capsule) (Utilities|Array|MakeArray "ObjectTypeQuery1" "ObjectTypeQuery5" "ObjectTypeQuery3") 0))
      (if _returnvalue
        (Utilities|FlowControl|Delay 3.0)
        (CallFunction|Spawn)
        (else
          (bind _returnvalue_2 (Game|SpawnActorfromClass "/Game/Mordhau/Blueprints/Interactables/SiegeEngines/BP_Mortar.BP_Mortar_C" (Transformation|GetWorldTransform (Variables|Default|GetCapsule)) "AlwaysSpawn" 0 0))
          (if (> _overridelookuplimit 0.0)
            (Variables|/Game/Mordhau/Blueprints/Interactables/SiegeEngines/BP_Mortar.BP_Mortar_C|SetReplicatedLookUpCap _returnvalue_2 _overridelookuplimit))
          (if (> _overrideturnlimit 0.0)
            (Variables|/Game/Mordhau/Blueprints/Interactables/SiegeEngines/BP_Mortar.BP_Mortar_C|SetReplicatedTurnCap _returnvalue_2 _overrideturnlimit))
          (if (> (Variables|Default|GetRespawnTime) 0.0)
            (EventDispatchers|AssignOnCharacterDied _returnvalue_2 (delegate Custom|OnBallistaDied))))))))

(event EventBeginPlay
  (Networking|SwitchHasAuthority
    (:Authority
      (Utilities|FlowControl|Sequence
        (:then_0
          (bind _asmordhau_game_mode (Utilities|Casting|CastToMordhauGameMode (Game|GetGameMode)))
          (Variables|Default|SetRespawnTime (Variables|/Script/Mordhau.MordhauGameMode|GetBallistaRespawnTime _asmordhau_game_mode)))
        (:then_1
          (CallFunction|Spawn))))))

(fn ConstructionScript)