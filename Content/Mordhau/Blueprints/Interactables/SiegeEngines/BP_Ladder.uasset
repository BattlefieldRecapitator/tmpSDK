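; Climbable ladder interactable that treats climbing as driving a vehicle.
; On interaction it spawns a BP_LadderMover at the point on the start-to-end line closest to the character, which then drives it.
; CanInteract requires vehicle permission and the parent check for valid characters.
; Only locally controlled characters get the position test, which allows entry near the top or below a local X limit.
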(event EventBeginPlay)

(event EventActorBeginOverlap
  (params (OtherActor :type Actor%20Object%20Reference)))

(event EventTick
  (params (DeltaSeconds :type Float%20%28single-precision%29)))

(event EventOnInteractionStart
  (params (Character :type Mordhau%20Character%20Object%20Reference))
  (bind _returnvalue (Game|SpawnActorfromClass "/Game/Mordhau/Blueprints/Interactables/SiegeEngines/BP_LadderMover.BP_LadderMover_C" (Math|Transform|MakeTransform (Class|MordhauUtilityLibrary|ClosestPointonLine (Transformation|GetWorldLocation (Variables|Default|GetLadderStart)) (Transformation|GetWorldLocation (Variables|Default|GetLadderEnd)) (Transformation|GetActorLocation Character)) (Transformation|GetActorRotation)) "AlwaysSpawn" 0 0))
  (Variables|/Game/Mordhau/Blueprints/Interactables/SiegeEngines/BP_LadderMover.BP_LadderMover_C|SetLadder _returnvalue self)
  (Class|MordhauVehicle|StartDriving _returnvalue Character))

(fn ConstructionScript
  (|CallParentFunction))

(fn CanInteract
  (params (Character :type Mordhau%20Character%20Object%20Reference))
  (bind _returnvalue (Transformation|GetActorLocation Character))
  (Utilities|IsValid Character
    (:Is%20Valid
      (if (Variables|/Script/Mordhau.MordhauCharacter|GetbAllowVehicles Character)
        (if (stale _returnvalue)
          (if (stale _returnvalue)
            (if (> (.Z (Math|Vector|BreakVector _returnvalue)) (- (.Z (Math|Vector|BreakVector (Transformation|GetWorldLocation (Variables|Default|GetLadderEnd)))) 75.0))
              _
              (else
                (return (< (.X (Math|Vector|BreakVector (Math|Transform|InverseTransformLocation (Transformation|GetActorTransform) _returnvalue))) 1e+01)))))
          (return true)
          (else
            _)))
      (return false))
    (:Is%20Not%20Valid
      (return (stale _returnvalue)))))