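; Drivable catapult siege engine with steering, aiming, a mouse-wheel adjusted arm draw and ragdoll on death.
; Firing runs a timed state machine (release, projectile spawn, pause, reload), with OnRep_State setting stage durations, sounds and projectile visibility.
; BPLODTick animates ArmTarget from the stage or replicated draw and drives the arm movement sound.
; On authority, nav obstacles stop affecting navigation while driven or once destroyed.
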(event Custom|RaiseArm
  (CallFunction|AdjustArm (* (Class|KismetSystemLibrary|MakeLiteralInteger 25) -1)))

(event Custom|LowerArm
  (CallFunction|AdjustArm (Class|KismetSystemLibrary|MakeLiteralInteger 25)))

(event Custom|FireCatapult
  (if (== (Variables|Default|GetState) 0)
    (Variables|Default|SetFiredController (Pawn|GetController))
    (Variables|Default|SetState 1)
    (Utilities|FlowControl|Delay (Variables|Default|GetStageTotalTime))
    (bind _returnvalue (Game|SpawnActorfromClass "/Game/Mordhau/Blueprints/Interactables/SiegeEngines/BP_CatapultProjectile.BP_CatapultProjectile_C" (Transformation|GetSocketTransform (Variables|Character|GetMesh) "FireSocket" "RTS_World") "AlwaysSpawn" self 0))
    (Class|MordhauProjectile|InitializeProjectile _returnvalue (Variables|Default|GetFiredController) false self)
    (Class|MordhauProjectile|Fire _returnvalue)
    (Variables|Default|SetState 2)
    (Utilities|FlowControl|Delay (Variables|Default|GetStageTotalTime))
    (Variables|Default|SetState 3)
    (Utilities|FlowControl|Delay (Variables|Default|GetStageTotalTime))
    (Variables|Default|SetState 0)))

(event EventBeginPlay
  (bind _mesh (Variables|Character|GetMesh))
  (Utilities|FlowControl|Sequence
    (:then_0
      (bind _returnvalue (Rendering|Material|CreateDynamicMaterialInstance _mesh 0 (Rendering|Material|GetMaterial _mesh 0) "None" :!class /Script/Engine.PrimitiveComponent))
      (Class|AdvancedCharacter|RegisterMaterialtoDissolve _returnvalue))
    (:then_1
      (Networking|SwitchHasAuthority
        (:Authority
          (Class|MordhauUtilityLibrary|SetCanEverAffectNavigation (Variables|Default|GetCapsuleComponent) false))))))

(event EventOnStartedDriving
  (params (Character :type Mordhau%20Character%20Object%20Reference))
  (|CallParentFunction Character)
  (Networking|SwitchHasAuthority
    (:Authority
      (Class|MordhauUtilityLibrary|SetCanEverAffectNavigation (Variables|Default|GetNavObstacle1) false)
      (Class|MordhauUtilityLibrary|SetCanEverAffectNavigation (Variables|Default|GetNavObstacle2) false))))

(event EventUnpossessed
  (params (OldController :type Controller%20Object%20Reference))
  (|CallParentFunction OldController))

(event EventBPLODTick
  (params (DeltaTime :type Float%20%28single-precision%29))
  (bind _loadedarmmin (Variables|Default|GetLoadedArmMin))
  (bind _state (Variables|Default|GetState))
  (|CallParentFunction DeltaTime)
  (Utilities|FlowControl|Sequence
    (:then_0
      (if (> _state 0)
        (Variables|Default|SetStageRemainingTime (Math|Float|Max(Float) (- (Variables|Default|GetStageRemainingTime) DeltaTime) 0.0))
        (switch int (Math|Conversions|ToInteger(Byte) _state)
          (:1
            (Variables|Default|SetArmTarget (Math|Float|Lerp 0.0 (Variables|Default|GetArmFrom) (/ (Variables|Default|GetStageRemainingTime) (Variables|Default|GetStageTotalTime)))))
          (:2
            (Variables|Default|SetArmTarget 0.0)
            (Networking|SwitchHasAuthority
              (:Authority
                (Variables|Default|SetReplicatedArm 0))))
          (:3
            (Variables|Default|SetArmTarget (Math|Interpolation|Ease "EaseIn" (/ (Variables|Default|GetStageRemainingTime) (Variables|Default|GetStageTotalTime)) (Variables|Default|GetLoadedArmMin) 0.0 2.0))))
        (else
          (Variables|Default|SetArmTarget (Math|Interpolation|FInterptoConstant (Variables|Default|GetArmTarget) (+ _loadedarmmin (* (- 1.0 _loadedarmmin) (/ (Math|Conversions|ToFloat(Byte) (Variables|Default|GetReplicatedArm)) 1e+02))) DeltaTime 0.125)))))
    (:then_1
      (if (and (> (/ (Math|Float|Absolute(Float) (- (Variables|Default|GetArmTarget) (Variables|Default|GetLastArmTarget))) DeltaTime) 0.05) (< (/ (Math|Float|Absolute(Float) (- (Variables|Default|GetArmTarget) (Variables|Default|GetLastArmTarget))) DeltaTime) 1e+01))
        (Utilities|IsValid (Variables|Default|GetLastArmPullSound)
          (:Is%20Not%20Valid
            (bind _returnvalue (Audio|SpawnSoundAttached "/Game/Mordhau/Audio/Cues/Siege/SC_Catapult_ArmMovement.SC_Catapult_ArmMovement" (Variables|Character|GetMesh) "Root" "0, 0, 0" "0, 0, 0" "SnapToTarget" true 1.0 1.0 0.0 0 0))
            (Variables|Default|SetLastArmPullSound _returnvalue)))
        (else
          (Utilities|IsValid (Variables|Default|GetLastArmPullSound)
            (:Is%20Valid
              (Audio|Components|Audio|FadeOut (Variables|Default|GetLastArmPullSound) 0.2 0.0 :!class /Script/Engine.AudioComponent)
              (Variables|Default|SetLastArmPullSound 0))))))
    (:then_2
      (Variables|Default|SetLastArmTarget (Variables|Default|GetArmTarget)))))

(event EventOnStoppedDriving
  (params (Character :type Mordhau%20Character%20Object%20Reference))
  (|CallParentFunction Character)
  (Networking|SwitchHasAuthority
    (:Authority
      (Class|MordhauUtilityLibrary|SetCanEverAffectNavigation (Variables|Default|GetNavObstacle1) true)
      (Class|MordhauUtilityLibrary|SetCanEverAffectNavigation (Variables|Default|GetNavObstacle2) true))))

(event EventOnCosmeticHit
  (params (DamageType :type EMordhauDamageType%20Enum :default "Generic") (SubType :type Byte :default 0) (Hit :type Hit%20Result%20Structure%20%28by%20ref%29) (Agent :type Actor%20Object%20Reference))
  (bind (_bblockinghit _binitialoverlap _time _distance _location _impactpoint _normal _impactnormal _physmat _hitactor _hitcomponent _hitbonename) (Collision|BreakHitResult Hit))
  (bind _self self)
  (|CallParentFunction DamageType SubType Hit Agent)
  (Class|PrimitiveComponent|AddForceatLocation (Variables|Character|GetMesh) (* (CallFunction|ComputeRagdollForce Agent DamageType SubType 0 _self _self) 1e+02) _impactpoint _hitbonename))

(event EventOnDied
  (params (Angle :type Float%20%28single-precision%29) (Type :type EMordhauDamageType%20Enum :default "Generic") (SubType :type Byte :default 0) (bone :type Name%20%28by%20ref%29 :default "None") (Point :type Vector%20%28by%20ref%29 :default "0, 0, 0") (Source :type Actor%20Object%20Reference) (Agent :type Actor%20Object%20Reference))
  (bind _self self)
  (bind _lastarmpullsound (Variables|Default|GetLastArmPullSound))
  (|CallParentFunction Angle Type SubType bone Point Source Agent)
  (Class|AdvancedCharacter|StartRagdoll)
  (Class|PrimitiveComponent|AddForceatLocation (Variables|Character|GetMesh) (* (CallFunction|ComputeRagdollForce Agent Type SubType 0 _self _self) 1e+02) Point bone)
  (Utilities|FlowControl|Sequence
    (:then_0
      (Utilities|IsValid _lastarmpullsound
        (:Is%20Valid
          (Audio|Components|Audio|FadeOut _lastarmpullsound 0.3 0.0 :!class /Script/Engine.AudioComponent))))
    (:then_1
      (Development|SetHiddeninGame (Variables|Default|GetProjectile) true false))
    (:then_2
      (Networking|SwitchHasAuthority
        (:Authority
          (Class|MordhauUtilityLibrary|SetCanEverAffectNavigation (Variables|Default|GetNavObstacle1) false)
          (Class|MordhauUtilityLibrary|SetCanEverAffectNavigation (Variables|Default|GetNavObstacle2) false))))))

(event EventUpdateFPCamerafor
  (params (Character :type Mordhau%20Character%20Object%20Reference) (DeltaSeconds :type Float%20%28single-precision%29) (bRotationOnly :type Boolean))
  (|CallParentFunction Character DeltaSeconds bRotationOnly)
  (Class|MordhauCharacter|UpdateFPCamera Character DeltaSeconds (Variables|Default|GetLookUpValue) bRotationOnly (Math|Rotator|MakeRotator 0.0 0.0 (Variables|Default|GetSecondaryTurnValue))))

(event Input|ActionEvents|InputActionFire
  (params (Key :type Key%20Structure))
  (:Pressed
    (CallFunction|FireCatapult)))

(event Input|ActionEvents|InputActionCycleCamera
  (params (Key :type Key%20Structure))
  (bind _driver (Variables|Default|GetDriver))
  (:Pressed
    (Utilities|IsValid _driver
      (:Is%20Valid
        (Class|MordhauCharacter|CycleCamera _driver)))))

(event Input|AxisEvents|InputAxisMoveRight
  (params (AxisValue :type Float%20%28single-precision%29))
  (Class|AdvancedCharacter|Turn (Math|Float|Clamp(Float) AxisValue -1.0) false))

(event Input|AxisEvents|InputAxisLookUp
  (params (AxisValue :type Float%20%28single-precision%29))
  (Class|AdvancedCharacter|LookUp AxisValue false))

(event Input|AxisEvents|InputAxisTurnRight
  (params (AxisValue :type Float%20%28single-precision%29))
  (Class|MordhauVehicle|SecondaryTurn AxisValue false))

(event Input|MouseEvents|MouseWheelDown
  (params (Key :type Key%20Structure))
  (bind _returnvalue (Utilities|Time|GetRealTimeSeconds))
  (:Pressed
    (if (and (== (Variables|Default|GetState) 0) (< (+ (Variables|Default|GetLastMouseWheelDownTime) (Math|Float|MakeLiteralFloat 0.4)) _returnvalue))
      (CallFunction|LowerArm)
      (Variables|Default|SetLastMouseWheelDownTime _returnvalue))))

(event Input|MouseEvents|MouseWheelUp
  (params (Key :type Key%20Structure))
  (bind _returnvalue (Utilities|Time|GetRealTimeSeconds))
  (:Pressed
    (if (and (== (Variables|Default|GetState) 0) (< (+ (Variables|Default|GetLastMouseWheelUpTime) (Math|Float|MakeLiteralFloat 0.4)) _returnvalue))
      (CallFunction|RaiseArm)
      (Variables|Default|SetLastMouseWheelUpTime _returnvalue))))

(fn ConstructionScript
  (bind _backcapsule (Variables|Default|GetBackCapsule))
  (|CallParentFunction)
  (Variables|Default|SetArmTarget (Variables|Default|GetLoadedArmMin))
  (bind _aspseudo_vehicle_movement_component (Utilities|Casting|CastToPseudoVehicleMovementComponent (Variables|Character|GetCharacterMovement)))
  (Variables|/Script/Mordhau.PseudoVehicleMovementComponent|SetSecondaryComponents _aspseudo_vehicle_movement_component (Utilities|Array|MakeArray (Variables|Default|GetBox) (Variables|Default|GetBox1) _backcapsule))
  (Variables|/Script/Mordhau.PseudoVehicleMovementComponent|SetSecondaryStepCapableComponents _aspseudo_vehicle_movement_component (Utilities|Array|MakeArray _backcapsule))
  (Transformation|AttachComponentToComponent (Variables|Default|GetProjectile) (Variables|Character|GetMesh) "Projectile" "SnapToTarget" "SnapToTarget" "KeepWorld" false))

(fn OnRepState
  (bind _mesh (Variables|Character|GetMesh))
  (bind _replicatedarm (Variables|Default|GetReplicatedArm))
  (bind _returnvalue (Math|Conversions|ToFloat(Byte) _replicatedarm))
  (bind _returnvalue_2 (/ _returnvalue 1e+02))
  (if (not (stale _returnvalue))
    (Utilities|FlowControl|Sequence
      (:then_0
        (switch int (Math|Conversions|ToInteger(Byte) (Variables|Default|GetState))
          (:0
            (Audio|SpawnSoundAttached "/Game/Mordhau/Audio/Cues/Siege/SC_Catapult_Reloaded.SC_Catapult_Reloaded" _mesh "Projectile" "0, 0, 0" "0, 0, 0" "SnapToTarget" true 1.0 1.0 0.0 0 0))
          (:1
            (Variables|Default|SetStageTotalTime 0.2)
            (Variables|Default|SetArmFrom (Variables|Default|GetArmTarget))
            (Audio|SpawnSoundAttached "/Game/Mordhau/Audio/Cues/Siege/SC_Catapult_Lever.SC_Catapult_Lever" _mesh "Lever" "0, 0, 0" "0, 0, 0" "SnapToTarget" true 1.0 1.0 0.0 0 0)
            (bind _returnvalue_3 (Audio|SpawnSoundAttached "/Game/Mordhau/Audio/Cues/Siege/SC_Catapult_Woosh.SC_Catapult_Woosh" _mesh "Projectile" "0, 0, 0" "0, 0, 0" "SnapToTarget" true 1.0 1.0 0.0 0 0))
            (Utilities|IsValid _returnvalue_3
              (:Is%20Valid
                (Audio|Parameter|SetFloatParameter _returnvalue_3 "ShotPower" _returnvalue_2 :!class /Script/Engine.AudioComponent))))
          (:2
            (Variables|Default|SetStageTotalTime 4.0)
            (bind _returnvalue_4 (Audio|SpawnSoundAttached "/Game/Mordhau/Audio/Cues/Siege/SC_Catapult_ArmHit.SC_Catapult_ArmHit" _mesh "Projectile" "0, 0, 0" "0, 0, 0" "SnapToTarget" true 1.0 1.0 0.0 0 0))
            (Utilities|IsValid _returnvalue_4
              (:Is%20Valid
                (Audio|Parameter|SetFloatParameter _returnvalue_4 "ShotPower" _returnvalue_2 :!class /Script/Engine.AudioComponent))))
          (:3
            (Variables|Default|SetStageTotalTime 6.0))))
      (:then_1
        (Development|SetHiddeninGame (Variables|Default|GetProjectile) (>= (Variables|Default|GetState) 2) false))
      (:then_2
        (Variables|Default|SetStageRemainingTime (Variables|Default|GetStageTotalTime))))))

(fn AdjustArm
  (params (Delta :type Integer))
  (if (== (Variables|Default|GetState) 0)
    (Variables|Default|SetReplicatedArm (Math|Conversions|ToByte(Integer) (Math|Integer|Clamp(Integer) (+ Delta (Math|Conversions|ToInteger(Byte) (Variables|Default|GetReplicatedArm))) 0 100)))))

(fn PostProcessCameraPOV
  (params (InPOV :type POV%20Structure%20%28by%20ref%29))
  (bind _driver (Variables|Default|GetDriver))
  (Utilities|IsValid _driver
    (:Is%20Valid
      (if (Variables|/Script/Mordhau.MordhauCharacter|GetbIsFirstPerson _driver)
        _
        (else
          (return))))
    (:Is%20Not%20Valid
      _))
  (return))