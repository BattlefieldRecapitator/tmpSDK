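; Ballista bolt projectile that skewers what it kills, dragging the ragdoll or severed part along with it.
; On a kill, cosmetic logic queues dismemberment or ragdolls the character or horse, and a physics handle grabs the bone.
; Tick pins that handle to the bolt's StickyPoint socket.
; After a kill the bolt no longer attaches to pawns, and hits that don't stop it cap its speed.
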(event EventTick
  (params (DeltaSeconds :type Float%20%28single-precision%29))
  (|CallParentFunction DeltaSeconds)
  (Class|PhysicsHandleComponent|SetTargetLocationandRotation (Variables|Default|GetPhysicsHandle) (Transformation|GetSocketLocation (Variables|Default|GetSkeletalMeshComponent) "StickyPoint") (Transformation|GetActorRotation)))

(event EventOnPostDismemberedOther
  (params (bone :type Name%20%28by%20ref%29 :default "None") (Part :type Separated%20Body%20Part%20Object%20Reference))
  (bind _mesh (Variables|/Script/Mordhau.SeparatedBodyPart|GetMesh Part))
  (bind _returnvalue (Transformation|GetSocketRotation _mesh bone))
  (|CallParentFunction bone Part)
  (Physics|Components|PhysicsHandle|GrabComponentatLocationwithRotation (Variables|Default|GetPhysicsHandle) _mesh bone (+ (Transformation|GetSocketLocation _mesh bone) (* (Math|Vector|GetRightVector _returnvalue) -1e+01)) _returnvalue))

(event EventOnProjectileHit
  (params (HitLocation :type Vector%20%28by%20ref%29 :default "0, 0, 0") (HitNormal :type Vector%20%28by%20ref%29 :default "0, 0, 0") (BounceForce :type Float%20%28single-precision%29) (Surface :type Byte :default 0) (bHasHitWorld :type Boolean) (bHasStopped :type Boolean))
  (bind _projectilemovement (Variables|Default|GetProjectileMovement))
  (|CallParentFunction HitLocation HitNormal BounceForce Surface bHasHitWorld bHasStopped)
  (if (not bHasStopped)
    (Game|Components|ProjectileMovement|SetVelocityinLocalSpace _projectilemovement (Math|Vector|UnrotateVector (Math|Vector|ClampVectorSize (Variables|/Script/Engine.MovementComponent|GetVelocity _projectilemovement) 0.0 1e+03) (Transformation|GetActorRotation)))))

(event EventOnUsedtoKillOther
  (params (Character :type Advanced%20Character%20Object%20Reference) (Type :type EMordhauDamageType%20Enum :default "Generic") (SubType :type Byte :default 0) (bone :type Name%20%28by%20ref%29 :default "None") (Point :type Vector%20%28by%20ref%29 :default "0, 0, 0") (Source :type Actor%20Object%20Reference))
  (bind _mesh (Variables|/Script/Engine.Character|GetMesh Character))
  (|CallParentFunction Character Type SubType bone Point Source)
  (Variables|Default|SetDoNotAttachToPawns true)
  (Networking|CanExecuteCosmeticEvents
    (:True
      (bind _asmordhau_character (Utilities|Casting|CastToMordhauCharacter Character)
        (:then
          (bind _returnvalue (Class|MordhauCharacter|CanDismember _asmordhau_character bone))
          (if _returnvalue
            (bind _returnvalue_2 (Class|MordhauCharacter|QueueDismember _asmordhau_character bone false false (Math|Vector|MakeVector 0.0 0.0 0.0) self))
            (if (not _returnvalue_2)
              (Class|AdvancedCharacter|StartRagdoll Character :!label _label)
              (Physics|Components|PhysicsHandle|GrabComponentatLocationwithRotation (Variables|Default|GetPhysicsHandle) _mesh bone (Transformation|GetSocketLocation _mesh bone) (Transformation|GetSocketRotation _mesh bone)))
            (else
              (goto _label))))
        (:CastFailed
          (Utilities|Casting|CastToHorse Character)
          (goto _label))))))

(fn ConstructionScript
  (|CallParentFunction))

(fn AttachProjectile
  (params (Hit :type Hit%20Result%20Structure%20%28by%20ref%29))
  (if (Variables|Default|GetDoNotAttachToPawns)
    (Utilities|Casting|CastToPawn (.HitActor (Collision|BreakHitResult Hit))
      (:then
        (return false))
      (:CastFailed
        _)))
  (bind _returnvalue (|CallParentFunction Hit))
  (return _returnvalue))