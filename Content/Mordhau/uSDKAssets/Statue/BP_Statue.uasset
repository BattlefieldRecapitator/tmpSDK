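; BP_Statue is a placeable statue that displays a posed Mordhau character above a plaque, styled from a chosen preset.
; The construction script maps the preset to a character profile and sets its plaque texture through a dynamic material.
; BeginPlay spawns a real BP_MordhauCharacter at SpawnPoint, freezes it in the selected single-node animation pose, applies the profile with equipment, then disables movement and mesh collision.
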(event EventBeginPlay
  (bind _returnvalue (Class|MordhauUtilityLibrary|GetMordhauSingleton))
  (bind _returnvalue_2 (Game|SpawnActorfromClass "/Game/Mordhau/Blueprints/Characters/BP_MordhauCharacter.BP_MordhauCharacter_C" (Transformation|GetWorldTransform (Variables|Default|GetSpawn%20point)) "AlwaysSpawn" 0 0))
  (CallFunction|PoseStatue _returnvalue_2)
  (Audio|Components|Audio|Play (Variables|/Script/Engine.Character|GetMesh _returnvalue_2) false)
  (Utilities|IsValid _returnvalue
    (:Is%20Valid
      (Class|MordhauSingleton|ApplyProfileto _returnvalue (Variables|Default|GetProfile) _returnvalue_2 0 true)
      (Variables|/Script/Mordhau.MordhauCharacter|SetLeftHandEquipment _returnvalue_2 (Utilities|Array|Get(acopy) (Variables|/Script/Mordhau.MordhauCharacter|GetEquipment _returnvalue_2) 2))
      (Variables|/Script/Mordhau.MordhauCharacter|SetRightHandEquipment _returnvalue_2 (Utilities|Array|Get(acopy) (Variables|/Script/Mordhau.MordhauCharacter|GetEquipment _returnvalue_2) 1))
      (Pawn|Components|CharacterMovement|DisableMovement (Variables|/Script/Engine.Character|GetCharacterMovement _returnvalue_2))
      (Collision|SetCollisionEnabled (Variables|/Script/Engine.Character|GetMesh _returnvalue_2) "NoCollision"))))

(fn ConstructionScript
  (bind _staticmesh (Variables|Default|GetStaticMesh))
  (CallFunction|Presets (Variables|Default|GetPreset))
  (bind _returnvalue (Rendering|Material|CreateDynamicMaterialInstance _staticmesh 0 (Rendering|Material|GetMaterial _staticmesh 0) "None" :!class /Script/Engine.PrimitiveComponent))
  (Rendering|Material|SetTextureParameterValue _returnvalue "Plaque" (Variables|Default|GetPlaqueTexture)))

(fn Presets
  (params (Preset :type Statues%20Enum :default "NewEnumerator0"))
  (bind _presetprofiles (Variables|Default|GetPresetProfiles))
  (switch Utilities|FlowControl|Switch|SwitchonStatues Preset
    (:NewEnumerator0
      (Variables|Default|SetProfile (.Value (Utilities|Map|Find _presetprofiles "TheMattman")))
      (Variables|Default|SetPlaqueTexture "/Game/Mordhau/uSDKAssets/Statue/MattPlaque.MattPlaque"))
    (:NewEnumerator1
      (Variables|Default|SetProfile (.Value (Utilities|Map|Find _presetprofiles "Battlefield")))
      (Variables|Default|SetPlaqueTexture "/Game/Mordhau/uSDKAssets/Statue/BattlefieldPlaque.BattlefieldPlaque"))
    (:NewEnumerator2
      (Variables|Default|SetProfile (.Value (Utilities|Map|Find _presetprofiles "2Cool")))
      (Variables|Default|SetPlaqueTexture "/Game/Mordhau/uSDKAssets/Statue/2coolPlaque.2coolPlaque"))))

(fn PoseStatue
  (params (Statue :type BP%20Mordhau%20Character%20Object%20Reference))
  (bind _mesh (Variables|/Script/Engine.Character|GetMesh Statue))
  (Components|Animation|SetAnimationMode _mesh "AnimationSingleNode")
  (switch Utilities|FlowControl|Switch|SwitchonPoses (Variables|Default|GetPose)
    (:NewEnumerator0
      (Components|Animation|OverrideAnimationData _mesh "/Game/Mordhau/Animations/RawClips/Misc/Poses/GreatswordPose.GreatswordPose" true true 0.5 1.0))
    (:NewEnumerator1
      (Components|Animation|OverrideAnimationData _mesh "/Game/Mordhau/Animations/RawClips/Misc/Poses/LongbowPose.LongbowPose" true true 1.0 1.0))
    (:NewEnumerator2
      (Components|Animation|OverrideAnimationData _mesh "/Game/Mordhau/Animations/RawClips/Misc/Poses/LutePose.LutePose" true true 1.0 1.0))
    (:NewEnumerator3
      (Components|Animation|OverrideAnimationData _mesh "/Game/Mordhau/Animations/RawClips/Misc/Poses/OnehandBuckler.OnehandBuckler" true true 1.0 1.0))
    (:NewEnumerator4
      (Components|Animation|OverrideAnimationData _mesh "/Game/Mordhau/Animations/RawClips/Misc/Poses/Pose_BeartrapLean.Pose_BeartrapLean" true true 1.0 1.0))
    (:NewEnumerator5
      (Components|Animation|OverrideAnimationData _mesh "/Game/Mordhau/Animations/RawClips/Misc/Poses/Pose_FoldedArms.Pose_FoldedArms" true true 1.0 1.0))
    (:NewEnumerator6
      (Components|Animation|OverrideAnimationData _mesh "/Game/Mordhau/Animations/RawClips/Misc/Poses/Pose_HandHip.Pose_HandHip" true true 1.0 1.0))
    (:NewEnumerator7
      (Components|Animation|OverrideAnimationData _mesh "/Game/Mordhau/Animations/RawClips/Misc/Poses/Pose_KiteShieldStand.Pose_KiteShieldStand" true true 1.0 1.0))
    (:NewEnumerator8
      (Components|Animation|OverrideAnimationData _mesh "/Game/Mordhau/Animations/RawClips/Misc/Poses/Pose_HeaterShieldStand.Pose_HeaterShieldStand" true true 1.0 1.0))
    (:NewEnumerator9
      (Components|Animation|OverrideAnimationData _mesh "/Game/Mordhau/Animations/RawClips/Misc/Poses/Pose_PoleStand.Pose_PoleStand" true true 1.0 1.0))
    (:NewEnumerator10
      (Components|Animation|OverrideAnimationData _mesh "/Game/Mordhau/Animations/RawClips/Misc/Poses/Pose_PoleStandFlipped.Pose_PoleStandFlipped" true true 1.0 1.0))
    (:NewEnumerator11
      (Components|Animation|OverrideAnimationData _mesh "/Game/Mordhau/Animations/RawClips/Misc/Poses/Pose_ScytheStand.Pose_ScytheStand" true true 1.0 1.0))
    (:NewEnumerator12
      (Components|Animation|OverrideAnimationData _mesh "/Game/Mordhau/Animations/RawClips/Misc/Poses/Pose_ShoulderRestCrossbow.Pose_ShoulderRestCrossbow" true true 1.0 1.0))
    (:NewEnumerator13
      (Components|Animation|OverrideAnimationData _mesh "/Game/Mordhau/Animations/RawClips/Misc/Poses/Pose_ShoulderRestPole.Pose_ShoulderRestPole" true true 1.0 1.0))
    (:NewEnumerator14
      (Components|Animation|OverrideAnimationData _mesh "/Game/Mordhau/Animations/RawClips/Misc/Poses/Pose_ShoulderRestSword.Pose_ShoulderRestSword" true true 1.0 1.0))
    (:NewEnumerator15
      (Components|Animation|OverrideAnimationData _mesh "/Game/Mordhau/Animations/RawClips/Misc/Poses/Pose_ShoulderRestWaraxe.Pose_ShoulderRestWaraxe" true true 1.0 1.0))
    (:NewEnumerator16
      (Components|Animation|OverrideAnimationData _mesh "/Game/Mordhau/Animations/RawClips/Misc/Poses/Pose_SpearStand.Pose_SpearStand" true true 1.0 1.0))
    (:NewEnumerator17
      (Components|Animation|OverrideAnimationData _mesh "/Game/Mordhau/Animations/RawClips/Misc/Poses/Pose_SwordBack.Pose_SwordBack" true true 1.0 1.0))
    (:NewEnumerator18
      (Components|Animation|OverrideAnimationData _mesh "/Game/Mordhau/Animations/RawClips/Misc/Poses/Pose_SwordBastard.Pose_SwordBastard" true true 1.0 1.0))
    (:NewEnumerator19
      (Components|Animation|OverrideAnimationData _mesh "/Game/Mordhau/Animations/RawClips/Misc/Poses/Pose_SwordLean.Pose_SwordLean" true true 1.0 1.0))
    (:NewEnumerator20
      (Components|Animation|OverrideAnimationData _mesh "/Game/Mordhau/Animations/RawClips/Misc/Poses/Pose_SwordStand.Pose_SwordStand" true true 1.0 1.0))
    (:NewEnumerator21
      (Components|Animation|OverrideAnimationData _mesh "/Game/Mordhau/Animations/RawClips/Misc/Poses/Pose_SwordStand2.Pose_SwordStand2" true true 1.0 1.0))
    (:NewEnumerator22
      (Components|Animation|OverrideAnimationData _mesh "/Game/Mordhau/Animations/RawClips/Misc/Poses/Pose_Toolbox.Pose_Toolbox" true true 1.0 1.0))
    (:NewEnumerator23
      (Components|Animation|OverrideAnimationData _mesh "/Game/Mordhau/Animations/RawClips/Misc/Poses/RapierPose.RapierPose" true true 1.0 1.0))
    (:NewEnumerator24
      (Components|Animation|OverrideAnimationData _mesh "/Game/Mordhau/Animations/RawClips/Misc/Poses/SingleAxePose.SingleAxePose" true true 1.0 1.0))))