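; Test interactable spawner that toggles a single AI wolf on and off.
; On interaction it spawns BP_WolfCharacter with WolfBT at the Spawnpoint, sets its mesh to SK_Wolf_UDK and plays the spawner's skeletal mesh animation forward.
; Interacting while that wolf exists and Flipped is set destroys it and plays the animation in reverse.
; If the stored wolf is no longer valid, interaction spawns a new one regardless of Flipped.
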(event EventBeginPlay
  (|CallParentFunction) ; This node is disabled and will not be called.\nDrag off pins to build functionality.
)

(event Collision|EventActorBeginOverlap
  (params (OtherActor :type Actor%20Object%20Reference)))

(event EventTick
  (params (DeltaSeconds :type Float%20%28single-precision%29))
  (|CallParentFunction DeltaSeconds) ; This node is disabled and will not be called.\nDrag off pins to build functionality.
)

(event EventOnInteractionStart
  (params (Character :type Mordhau%20Character%20Object%20Reference))
  (bind _spawnpoint (Variables|Default|GetSpawnpoint))
  (bind _skeletalmesh (Variables|Default|GetSkeletalMesh))
  (bind _skeletalmesh_2 (Variables|Default|GetSkeletalMesh))
  (bind _returnvalue (Transformation|GetWorldTransform _spawnpoint))
  (Utilities|IsValid (Variables|Default|GetDog)
    (:Is%20Valid
      (if (Variables|Default|GetFlipped)
        (Actor|DestroyActor (Variables|Default|GetDog))
        (Components|Timeline|SetPlayRate _skeletalmesh -1.0)
        (Audio|Components|Audio|Play _skeletalmesh false)
        (Variables|Default|SetFlipped false)
        (else
          (bind _returnvalue_2 (AI|SpawnAIFromClass "/Game/Mordhau/uSDKAssets/Test/Wolf/BP_WolfCharacter.BP_WolfCharacter_C" "/Game/Mordhau/uSDKAssets/Test/Wolf/WolfBT.WolfBT" (.location _returnvalue) (.rotation _returnvalue) false :!label _label))
          (Components|Timeline|SetPlayRate _skeletalmesh_2 1.0)
          (Audio|Components|Audio|Play _skeletalmesh_2 false)
          (Variables|Default|SetFlipped true)
          (bind _asbp_wolf_character (Utilities|Casting|CastToBP_WolfCharacter _returnvalue_2))
          (Variables|Default|SetDog _asbp_wolf_character)
          (Class|SkinnedMeshComponent|SetSkeletalMesh (Variables|/Script/Engine.Character|GetMesh _asbp_wolf_character) "/Game/Mordhau/uSDKAssets/Test/Wolf/SK_Wolf_UDK.SK_Wolf_UDK" false))))
    (:Is%20Not%20Valid
      (if (Variables|Default|GetFlipped)
        (goto _label)
        (else
          (goto _label))))))

(fn ConstructionScript
  (|CallParentFunction))